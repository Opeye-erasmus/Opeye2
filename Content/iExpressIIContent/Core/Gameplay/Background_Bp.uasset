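; Background actor that tints its mesh from colour settings in the System_Save game save.
; BeginPlay creates a dynamic material, sets its emissive intensity, prints the saved ABGColour and maps it to BaseColor.
; GetSystemSave returns the cached save, or loads it from its slot, or creates a new one if none exists.
; ChangeColor ignores its Color input and picks BaseColor from the cached save's AColorConfig instead.
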(event Custom|ChangeColor
  (params (color :type Linear%20Color%20Structure))
  (bind _mat (Variables|Default|Getmat))
  (Rendering|Material|SetScalarParameterValue _mat "EmissiveInt" 1.0 :!class /Script/Engine.MaterialInstanceDynamic)
  (Rendering|Material|SetVectorParameterValue _mat "BaseColor" (Utilities|Select :Index (Variables|/Game/OpeyeIIContent/Core/Data/System_Save.System_Save_C|GetA_ColorConfig (Variables|Default|Getsystem)) :NewEnumerator0 "(R=0.000000,G=0.000000,B=0.000000,A=1.000000)" :NewEnumerator1 "(R=0.000000,G=0.000000,B=0.000000,A=1.000000)" :NewEnumerator2 "(R=1.000000,G=1.000000,B=1.000000,A=1.000000)" :NewEnumerator3 "(R=0.000000,G=0.000000,B=0.000000,A=1.000000)" :NewEnumerator4 "(R=0.004777,G=0.035601,B=0.274677,A=1.000000)" :NewEnumerator5 "" :NewEnumerator6 "(R=0.318547,G=0.000000,B=0.318547,A=1.000000)") :!class /Script/Engine.MaterialInstanceDynamic))

(event EventBeginPlay
  (bind _returnvalue (Rendering|Material|CreateDynamicMaterialInstance "/Game/OpeyeIIContent/Art/Base/BaseMaterial.BaseMaterial" "None" "None" :!class /Script/Engine.KismetMaterialLibrary))
  (Variables|Default|Setmat _returnvalue)
  (Rendering|Material|SetMaterial (Variables|Default|Getbackground) 0 _returnvalue)
  (Rendering|Material|SetScalarParameterValue (Variables|Default|Getmat) "EmissiveInt" 1.0 :!class /Script/Engine.MaterialInstanceDynamic)
  (bind _systemsave (CallFunction|GetSystemSave))
  (Development|PrintString (Utilities|String|EnumtoString (Variables|/Game/OpeyeIIContent/Core/Data/System_Save.System_Save_C|GetA_BG_Colour _systemsave)))
  (Rendering|Material|SetVectorParameterValue (Variables|Default|Getmat) "BaseColor" (Utilities|Select :Index (Variables|/Game/OpeyeIIContent/Core/Data/System_Save.System_Save_C|GetA_BG_Colour _systemsave) :NewEnumerator0 "" :NewEnumerator1 "(R=1.000000,G=1.000000,B=1.000000,A=1.000000)" :NewEnumerator2 "(R=0.854902,G=0.062745,B=0.145098,A=1.000000)" :NewEnumerator3 "(R=1.000000,G=0.941177,B=0.360784,A=1.000000)" :NewEnumerator4 "(R=0.113725,G=0.196078,B=0.329412,A=1.000000)" :NewEnumerator5 "(R=0.980392,G=1.000000,B=1.000000,A=1.000000)") :!class /Script/Engine.MaterialInstanceDynamic))

(event Collision|EventActorBeginOverlap
  (params (OtherActor :type Actor%20Object%20Reference)))

(event EventTick
  (params (DeltaSeconds :type Float%20%28single-precision%29)))

(fn ConstructionScript)

(fn GetSystemSave
  (Utilities|IsValid (Variables|Default|GetSystem)
    (:Is%20Valid
      (return (Variables|Default|GetSystem)))
    (:Is%20Not%20Valid
      (bind _returnvalue (SaveGame|DoesSaveGameExist (CallFunction|GetSystemSaveName)))
      (if _returnvalue
        (bind _returnvalue_2 (SaveGame|LoadGamefromSlot (CallFunction|GetSystemSaveName)))
        (bind _assystem_save (Utilities|Casting|CastToSystem_Save _returnvalue_2)
          (:then
            (Variables|Default|SetSystem _assystem_save))
          (:CastFailed
            _))
        (else
          (bind _returnvalue_3 (SaveGame|CreateSaveGameObject "/Game/OpeyeIIContent/Core/Data/System_Save.System_Save_C"))
          (Variables|Default|SetSystem _returnvalue_3)))
      (return (Variables|Default|GetSystem)))))
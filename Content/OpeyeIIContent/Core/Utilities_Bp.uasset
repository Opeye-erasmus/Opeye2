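; Shared utility Blueprint for menu navigation, screen-to-world math, save handling and exercise enum conversion in an eye-exercise app.
; Navigation reuses or creates the next widget and registers it with Menu_Pwn.
; Screen points project onto a camera-facing plane at a given distance.
; A cached System_Save supplies the last user name for profile slots; profile saves first drop the oldest entry from any smooth pursuit, saccade or field-of-view history exceeding ten.
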(fn NavigatetoNextWidget
  (params (currentWidget :type User%20Widget%20Object%20Reference) (nextWidget :type User%20Widget%20Class%20Reference))
  (bind _returnvalue (Game|Player|GetPlayerPawn 0))
  (Utilities|FlowControl|Sequence
    (:then_0
      (Utilities|IsValid currentWidget
        (:Is%20Valid
          (Widget|RemovefromParent currentWidget))))
    (:then_1
      (bind _foundwidgets (Widget|GetAllWidgetsOfClass 0 nextWidget false))
      (if (> (Utilities|Array|Length _foundwidgets) 0)
        (UserInterface|Viewport|AddtoViewport (Utilities|Array|Get(acopy) _foundwidgets) 0)
        (bind _asmenu_pwn (Utilities|Casting|CastToMenu_Pwn _returnvalue)
          (:then
            (Default|SetCurrentWidget _asmenu_pwn (Utilities|Array|Get(acopy) _foundwidgets)))
          (:CastFailed
            _))
        (return (Utilities|Array|Get(acopy) _foundwidgets))
        (else
          (bind _returnvalue_2 (UserInterface|CreateWidget nextWidget (Game|GetPlayerController 0)))
          (UserInterface|Viewport|AddtoViewport _returnvalue_2 0)
          (bind _asmenu_pwn_2 (Utilities|Casting|CastToMenu_Pwn _returnvalue)
            (:then
              (Default|SetCurrentWidget _asmenu_pwn_2 _returnvalue_2))
            (:CastFailed
              _))
          (return _returnvalue_2))))))

(fn Screen2WorldCoordinates
  (params (CamaraLocation :type Vector) (ScreenPos :type Vector%202D%20Structure) (Distance :type Float%20%28single-precision%29))
  (bind _returnvalue (Game|GetPlayerController 0))
  (bind _returnvalue_2 (Viewport|GetViewportSize))
  (bind _returnvalue_3 (Game|GetPlayerController 0))
  (bind _returnvalue_4 (* Distance 3.0))
  (bind _worlddirection (Class|GameplayStatics|DeprojectScreentoWorld _returnvalue_3 ScreenPos))
  (bind _returnvalue_5 (/ _returnvalue_2 2.0))
  (bind _returnvalue_6 (* _worlddirection _returnvalue_4))
  (bind _worlddirection_2 (Class|GameplayStatics|DeprojectScreentoWorld _returnvalue _returnvalue_5))
  (bind _returnvalue_7 (* _worlddirection_2 Distance))
  (bind _returnvalue_8 (+ CamaraLocation _returnvalue_6))
  (bind _returnvalue_9 (+ CamaraLocation _returnvalue_7))
  (bind _returnvalue_10 (Class|KismetMathLibrary|MakePlanefromPointandNormal _returnvalue_9 _worlddirection_2))
  (bind (_t _intersection _returnvalue_11) (Class|KismetMathLibrary|LinePlaneIntersection CamaraLocation _returnvalue_8 _returnvalue_10))
  (if _returnvalue_11
    (return _intersection)
    (else
      (return _returnvalue_8))))

(fn GetSystemSaveName
  (return "System_Save"))

(fn UserNametoSaveFileName
  (params (NewParam :type String))
  (return (Utilities|String|Append NewParam "_userSave")))

(fn GetSystemSave
  (Utilities|IsValid (LocalVariables|GetSystem)
    (:Is%20Valid
      (return (LocalVariables|GetSystem)))
    (:Is%20Not%20Valid
      (bind _returnvalue (SaveGame|DoesSaveGameExist (CallFunction|GetSystemSaveName)))
      (if _returnvalue
        (bind _returnvalue_2 (SaveGame|LoadGamefromSlot (CallFunction|GetSystemSaveName)))
        (bind _assystem_save (Utilities|Casting|CastToSystem_Save _returnvalue_2)
          (:then
            (LocalVariables|SetSystem _assystem_save))
          (:CastFailed
            _))
        (else
          (bind _returnvalue_3 (SaveGame|CreateSaveGameObject "/Game/OpeyeIIContent/Core/Data/System_Save.System_Save_C"))
          (LocalVariables|SetSystem _returnvalue_3)))
      (return (LocalVariables|GetSystem)))))

(fn LoadUserProfile
  (bind _systemsave (CallFunction|GetSystemSave))
  (bind _returnvalue (SaveGame|LoadGamefromSlot (CallFunction|UserNametoSaveFileName (Utilities|String|ToString(Name) (Variables|/Game/OpeyeIIContent/Core/Data/System_Save.System_Save_C|GetlastUserName _systemsave)))))
  (bind _asuser_profile_save (Utilities|Casting|CastToUserProfile_Save _returnvalue))
  (return _asuser_profile_save))

(fn SaveUserProfile
  (params (NewParam :type User%20Profile%20Save%20Object%20Reference))
  (bind _save_trimmed (CallFunction|CheckEveryDataLength NewParam))
  (bind _systemsave (CallFunction|GetSystemSave))
  (bind _returnvalue (SaveGame|SaveGametoSlot _save_trimmed (CallFunction|UserNametoSaveFileName (Utilities|String|ToString(Name) (Variables|/Game/OpeyeIIContent/Core/Data/System_Save.System_Save_C|GetlastUserName _systemsave)))))
  (if _returnvalue
    (Development|PrintString 0 "saved")
    (else
      (Development|PrintString 0 "hell"))))

(fn SaveSystemSave
  (params (Save :type System%20Save%20Object%20Reference))
  (bind _newparam (CallFunction|GetSystemSaveName))
  (bind _returnvalue (SaveGame|SaveGametoSlot Save _newparam))
  (if _returnvalue
    (Development|PrintString 0 (Utilities|String|Append "Save in: " _newparam))
    (else
      (Development|PrintString 0 (Utilities|String|Append "Couldn't save: " _newparam))
      (Utilities|IsValid Save
        (:Is%20Valid
          (Development|PrintString 0 "save is valid"))
        (:Is%20Not%20Valid
          (Development|PrintString 0 "save is invalid"))))))

(fn CheckEveryDataLength
  (params (Save :type User%20Profile%20Save%20Object%20Reference))
  (bind _smoothpursuita_data (Variables|/Game/OpeyeIIContent/Core/Data/UserProfile_Save.UserProfile_Save_C|GetsmoothPursuitA_Data Save))
  (bind _smoothpursuitb_data (Variables|/Game/OpeyeIIContent/Core/Data/UserProfile_Save.UserProfile_Save_C|GetsmoothPursuitB_Data Save))
  (bind _smoothpursuitc_data (Variables|/Game/OpeyeIIContent/Core/Data/UserProfile_Save.UserProfile_Save_C|GetsmoothPursuitC_Data Save))
  (bind _smoothpursuitd_data (Variables|/Game/OpeyeIIContent/Core/Data/UserProfile_Save.UserProfile_Save_C|GetsmoothPursuitD_Data Save))
  (bind _saccadesa_data (Variables|/Game/OpeyeIIContent/Core/Data/UserProfile_Save.UserProfile_Save_C|GetsaccadesA_Data Save))
  (bind _saccadesb_data (Variables|/Game/OpeyeIIContent/Core/Data/UserProfile_Save.UserProfile_Save_C|GetsaccadesB_Data Save))
  (bind _saccadesc_data (Variables|/Game/OpeyeIIContent/Core/Data/UserProfile_Save.UserProfile_Save_C|GetsaccadesC_Data Save))
  (bind _saccadesd_data (Variables|/Game/OpeyeIIContent/Core/Data/UserProfile_Save.UserProfile_Save_C|GetsaccadesD_Data Save))
  (bind _fieldofviewa0_data (Variables|/Game/OpeyeIIContent/Core/Data/UserProfile_Save.UserProfile_Save_C|GetfieldOfViewA0_Data Save))
  (bind _fieldofviewa1_data (Variables|/Game/OpeyeIIContent/Core/Data/UserProfile_Save.UserProfile_Save_C|GetfieldOfViewA1_Data Save))
  (Utilities|FlowControl|Sequence
    (:then_0
      (if (> (Utilities|Array|Length _smoothpursuita_data) 10)
        (Utilities|Array|RemoveIndex _smoothpursuita_data)))
    (:then_1
      (if (> (Utilities|Array|Length _smoothpursuitb_data) 10)
        (Utilities|Array|RemoveIndex _smoothpursuitb_data)))
    (:then_2
      (if (> (Utilities|Array|Length _smoothpursuitc_data) 10)
        (Utilities|Array|RemoveIndex _smoothpursuitc_data)))
    (:then_3
      (if (> (Utilities|Array|Length _smoothpursuitd_data) 10)
        (Utilities|Array|RemoveIndex _smoothpursuitd_data)))
    (:then_4
      (if (> (Utilities|Array|Length _saccadesa_data) 10)
        (Utilities|Array|RemoveIndex _saccadesa_data)))
    (:then_5
      (if (> (Utilities|Array|Length _saccadesb_data) 10)
        (Utilities|Array|RemoveIndex _saccadesb_data)))
    (:then_6
      (if (> (Utilities|Array|Length _saccadesc_data) 10)
        (Utilities|Array|RemoveIndex _saccadesc_data)))
    (:then_7
      (if (> (Utilities|Array|Length _saccadesd_data) 10)
        (Utilities|Array|RemoveIndex _saccadesd_data)))
    (:then_8
      (if (> (Utilities|Array|Length _fieldofviewa0_data) 10)
        (Utilities|Array|RemoveIndex _fieldofviewa0_data)))
    (:then_9
      (if (> (Utilities|Array|Length _fieldofviewa1_data) 10)
        (Utilities|Array|RemoveIndex _fieldofviewa1_data)))
    (:then_10
      (return Save))))

(fn LevelEnumtoSmoothPursuitEnum
  (params (level :type Level_Enum%20Enum :default "NewEnumerator0"))
  (return (Utilities|Select :Index level :NewEnumerator0 "NewEnumerator0" :NewEnumerator1 "NewEnumerator1" :NewEnumerator2 "NewEnumerator2" :NewEnumerator3 "NewEnumerator4" :NewEnumerator4 "NewEnumerator5" :NewEnumerator5 "NewEnumerator6" :NewEnumerator6 "NewEnumerator7" :NewEnumerator7 "NewEnumerator8" :NewEnumerator8 "NewEnumerator9" :NewEnumerator9 "NewEnumerator10" :NewEnumerator10 "NewEnumerator11" :NewEnumerator11 "NewEnumerator12" :NewEnumerator12 "NewEnumerator13" :NewEnumerator13 "NewEnumerator14" :NewEnumerator14 "NewEnumerator15" :NewEnumerator15 "NewEnumerator16" :NewEnumerator16 "NewEnumerator17" :NewEnumerator17 "NewEnumerator18" :NewEnumerator18 "NewEnumerator19" :NewEnumerator19 "NewEnumerator20" :NewEnumerator20 "NewEnumerator21" :NewEnumerator21 "NewEnumerator22" :NewEnumerator22 "NewEnumerator23" :NewEnumerator23 "NewEnumerator0" :NewEnumerator24 "NewEnumerator0" :NewEnumerator25 "NewEnumerator0" :NewEnumerator26 "NewEnumerator0" :NewEnumerator27 "NewEnumerator0" :NewEnumerator28 "NewEnumerator0")))

(fn SmoothPursuitEnumtoLevelEnum
  (params (smooth :type SmoothPursuit_Enum%20Enum :default "NewEnumerator0"))
  (return (Utilities|Select :Index smooth :NewEnumerator0 "NewEnumerator0" :NewEnumerator1 "NewEnumerator1" :NewEnumerator2 "NewEnumerator2" :NewEnumerator4 "NewEnumerator3" :NewEnumerator5 "NewEnumerator4" :NewEnumerator6 "NewEnumerator5" :NewEnumerator7 "NewEnumerator6" :NewEnumerator8 "NewEnumerator7" :NewEnumerator9 "NewEnumerator8" :NewEnumerator10 "NewEnumerator9" :NewEnumerator11 "NewEnumerator10" :NewEnumerator12 "NewEnumerator11" :NewEnumerator13 "NewEnumerator12" :NewEnumerator14 "NewEnumerator13" :NewEnumerator15 "NewEnumerator14" :NewEnumerator16 "NewEnumerator15" :NewEnumerator17 "NewEnumerator16" :NewEnumerator18 "NewEnumerator17" :NewEnumerator19 "NewEnumerator18" :NewEnumerator20 "NewEnumerator19" :NewEnumerator21 "NewEnumerator20" :NewEnumerator22 "NewEnumerator21" :NewEnumerator23 "NewEnumerator22")))
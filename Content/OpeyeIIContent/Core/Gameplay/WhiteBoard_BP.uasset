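; Whiteboard Blueprint that records brush strokes into a render target and can be wiped clean.
; BeginPlay creates a dynamic brush material with size and opacity parameters, then clears the target to black.
; DrawOnWhiteboard packs the supplied location's X and Y into the brush's Position vector parameter and draws that material onto the target.
; Separate events resize the brush and clear the board.
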(event Custom|DrawOnWhiteboard
  (params (LocationToDraw :type Vector%202D%20Structure))
  (bind (_x _y) (Math|Vector2D|BreakVector2D LocationToDraw))
  (bind _brush (Variables|Default|GetBrush))
  (Rendering|Material|SetVectorParameterValue _brush "Position" (Utilities|Struct|MakeLinearColor _x _y 0.0 1.0) :!class /Script/Engine.MaterialInstanceDynamic)
  (Rendering|DrawMaterialtoRenderTarget "/Game/OpeyeIIContent/Art/PaintAndClean/WhiteBoard_RT.WhiteBoard_RT" _brush))

(event Custom|ChangeBrushSize
  (params (BrushSize :type Float%20%28single-precision%29))
  (bind _output_get (Variables|Default|SetBrushSize BrushSize))
  (Rendering|Material|SetScalarParameterValue (Variables|Default|GetBrush) "Size" _output_get :!class /Script/Engine.MaterialInstanceDynamic))

(event Custom|CleanBoard
  (Rendering|ClearRenderTarget2D "/Game/OpeyeIIContent/Art/PaintAndClean/WhiteBoard_RT.WhiteBoard_RT"))

(event EventBeginPlay
  (bind _returnvalue (Rendering|Material|CreateDynamicMaterialInstance "/Game/OpeyeIIContent/Art/PaintAndClean/Brush_Mat.Brush_Mat" "None" "None" :!class /Script/Engine.KismetMaterialLibrary))
  (bind _output_get (Variables|Default|SetBrush _returnvalue))
  (Rendering|Material|SetScalarParameterValue _output_get "Size" (Variables|Default|GetBrushSize) :!class /Script/Engine.MaterialInstanceDynamic)
  (Rendering|Material|SetScalarParameterValue _output_get "Opacity" (Variables|Default|GetBrushOpacity) :!class /Script/Engine.MaterialInstanceDynamic)
  (Rendering|ClearRenderTarget2D "/Game/OpeyeIIContent/Art/PaintAndClean/WhiteBoard_RT.WhiteBoard_RT"))

(event Collision|EventActorBeginOverlap
  (params (OtherActor :type Actor%20Object%20Reference)))

(event EventTick
  (params (DeltaSeconds :type Float%20%28single-precision%29)))

(fn ConstructionScript)
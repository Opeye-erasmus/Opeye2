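; SphereTargetResult_Bp is a sphere actor, named as a target result marker, whose material is set through a SetMaterial event.
; Helper functions compute a rotation toward the player pawn and convert an eye screen position to centered, normalized viewport coordinates.
; GetSystemSave lazily caches the System_Save, loading it from its slot or creating an unsaved instance when none exists.
; BeginPlay, the construction script and GetTarget are empty, and no graph here calls the helpers.
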(event Custom|SetMaterial
  (params (Material :type Material%20Interface%20Object%20Reference))
  (Rendering|Material|SetMaterial (Variables|Default|GetSphere) 0 Material))

(event EventBeginPlay)

(fn ConstructionScript)

(fn GetLookRotation
  (return (Math|Rotator|FindLookatRotation (Transformation|GetActorLocation) (Transformation|GetActorLocation (Game|Player|GetPlayerPawn 0)))))

(fn GetNormalizedPositionOfEye
  (params (A :type Vector%202D%20Structure))
  (bind _returnvalue (Viewport|GetViewportSize))
  (bind _returnvalue_2 (Class|WidgetLayoutLibrary|GetViewportScale))
  (bind (_x _y) (Math|Vector2D|BreakVector2D _returnvalue))
  (bind _returnvalue_3 (* A _returnvalue_2))
  (bind (_x_2 _y_2) (Math|Vector2D|BreakVector2D _returnvalue_3))
  (bind _returnvalue_4 (/ _y 2.0))
  (bind _returnvalue_5 (/ _x 2.0))
  (bind _returnvalue_6 (- _x_2 _returnvalue_5))
  (bind _returnvalue_7 (- _y_2 _returnvalue_4))
  (bind _returnvalue_8 (/ _returnvalue_6 _returnvalue_5))
  (bind _returnvalue_9 (/ _returnvalue_7 _returnvalue_4))
  (return _returnvalue_8 _returnvalue_9 (Math|Vector2D|MakeVector2D _returnvalue_8 _returnvalue_9)))

(fn GetSystemSave
  (Utilities|IsValid (Variables|Default|GetSystem)
    (:Is%20Valid
      (return (Variables|Default|GetSystem)))
    (:Is%20Not%20Valid
      (bind _returnvalue (SaveGame|DoesSaveGameExist (CallFunction|GetSystemSaveName)))
      (if _returnvalue
        (bind _returnvalue_2 (SaveGame|LoadGamefromSlot (CallFunction|GetSystemSaveName)))
        (bind _assystem_save (Utilities|Casting|CastToSystem_Save _returnvalue_2)
          (:then
            (Variables|Default|SetSystem _assystem_save))
          (:CastFailed
            _))
        (else
          (bind _returnvalue_3 (SaveGame|CreateSaveGameObject "/Game/OpeyeIIContent/Core/Data/System_Save.System_Save_C"))
          (Variables|Default|SetSystem _returnvalue_3)))
      (return (Variables|Default|GetSystem)))))

(fn GetTarget
  (return 0))
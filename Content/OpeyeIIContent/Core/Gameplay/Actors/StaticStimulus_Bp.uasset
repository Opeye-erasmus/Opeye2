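; StaticStimulus_Bp is a stationary gaze target for an eye-tracking exercise, colored from the saved color scheme.
; Tobii gaze focus or hit events feed HitManagerCmp, whose completion and full-track-loss callbacks notify the parent actor while not Viewed.
; A five-second timer reports a timeout to the FOV spawner.
; BeginPlay hides the halo and applies a dynamic material to the sphere and halo.
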(event OnComponentBeginOverlap(Box)
  (params (OverlappedComponent :type Primitive%20Component%20Object%20Reference) (OtherActor :type Actor%20Object%20Reference) (OtherComp :type Primitive%20Component%20Object%20Reference) (OtherBodyIndex :type Integer) (bFromSweep :type Boolean) (SweepResult :type Hit%20Result%20Structure%20%28by%20ref%29))
  ;[1 1 1] Jose: I have removed this connection
)

(event OnPrimitiveReceivedGazeFocus(TobiiGazeFocusable)
  (params (FocusedComponent :type Primitive%20Component%20Object%20Reference))
  ;[1 0 0] It is going to receive the call twice when using tobii
  (CallFunction|Hit))

(event Custom|EyesightIsTrackingMeAgain)

(event Custom|ExerciseWasCompleted
  (if (not (Variables|Default|Getviewed))
    (Class|ListenerInt|ListenedActorIsDone(Message) (Variables|Default|GetparentActor) self)
    (CallFunction|ResetCache)))

(event Custom|EyesightTrackWasLost)

(event Custom|EyetrackWasFullyLost
  (if (not (Variables|Default|Getviewed))
    (Class|ListenerInt|ListenedActorIsFullyLost(Message) (Variables|Default|GetparentActor) self)))

(event Custom|Timeout
  (if (not (< (Variables|Default|Getflags) 0))
    (bind _outactors (Actor|GetAllActorsOfClass "/Game/OpeyeIIContent/Core/Gameplay/Spawners/FOVActorSpawner_Bp.FOVActorSpawner_Bp_C"))
    (Default|StaticStimReachedTimeout (Utilities|Array|Get(acopy) _outactors) self)))

(event Custom|StopTimer
  (Utilities|Time|ClearandInvalidateTimerbyHandle (stale EventBeginPlay _returnvalue)))

(event Custom|ChangeHaloVisibility
  (params (visible :type Boolean))
  (Rendering|SetVisibility (Variables|Default|Gethalo) visible false))

(event Custom|ResetCache
  (Default|FullResetCache (Variables|Default|GetHitManager_Cmp)))

(event EventBeginPlay
  (bind _hitmanager_cmp (Variables|Default|GetHitManager_Cmp))
  (Rendering|SetVisibility (Variables|Default|Gethalo) false false)
  (bind _returnvalue (Utilities|Time|SetTimerbyEvent (delegate Custom|Timeout) 5.0))
  (EventDispatchers|BindEventtoTrackLossWarning _hitmanager_cmp (delegate Custom|EyesightTrackWasLost))
  (EventDispatchers|BindEventtoExerciseComplete _hitmanager_cmp (delegate Custom|ExerciseWasCompleted))
  (EventDispatchers|BindEventtoStartedBeingTracked _hitmanager_cmp (delegate Custom|EyesightIsTrackingMeAgain))
  (EventDispatchers|BindEventtoTrackFullyLostWarning _hitmanager_cmp (delegate Custom|EyetrackWasFullyLost))
  (CallFunction|ChangeStimulusColour))

(event EventTick
  (params (DeltaSeconds :type Float%20%28single-precision%29))
  (Variables|Default|SettimeElapsed (+ DeltaSeconds (Variables|Default|GettimeElapsed)))
  (Utilities|FlowControl|Delay 0.01)
  (Variables|Default|Setmilliseconds (+ (Variables|Default|Getmilliseconds) 1)))

(event EventSetParent
  (params (Actor :type Actor%20Object%20Reference))
  (Variables|Default|SetparentActor Actor))

(event EventHit
  (params (Hit%20Component%20Name :type String))
  ;[1 0 0] It is going to receive the call twice when using tobii
  (Default|ManageHit (Variables|Default|GetHitManager_Cmp)))

(fn ConstructionScript)

(fn ChangeStimulusColour
  (bind _sphere (Variables|Default|GetSphere))
  (bind _returnvalue (Rendering|Material|CreateDynamicMaterialInstance _sphere 0 "/Game/OpeyeIIContent/Art/Base/BaseMaterial.BaseMaterial" "None" :!class /Script/Engine.PrimitiveComponent))
  (Variables|Default|SetMat _returnvalue)
  (bind _systemsave (CallFunction|GetSystemSave))
  (Rendering|Material|SetVectorParameterValue _returnvalue "BaseColor" (Utilities|Select :Index (Variables|/Game/OpeyeIIContent/Core/Data/System_Save.System_Save_C|GetA_ColorConfig _systemsave) :NewEnumerator0 "(R=0.278894,G=1.000000,B=0.119538,A=1.000000)" :NewEnumerator1 "(R=1.000000,G=1.000000,B=1.000000,A=1.000000)" :NewEnumerator2 "(R=0.008568,G=0.127438,B=0.024158,A=1.000000)" :NewEnumerator3 "(R=0.913099,G=0.846873,B=0.000000,A=1.000000)" :NewEnumerator4 "(R=0.913099,G=0.846873,B=0.000000,A=1.000000)" :NewEnumerator5 "(R=1.000000,G=0.000000,B=0.000000,A=1.000000)" :NewEnumerator6 "(R=1.000000,G=1.000000,B=0.000000,A=1.000000)") :!class /Script/Engine.MaterialInstanceDynamic)
  (Rendering|Material|SetMaterial _sphere 0 (Variables|Default|GetMat)))

(fn GetSystemSave
  (Utilities|IsValid (Variables|Default|GetSystem)
    (:Is%20Valid
      (return (Variables|Default|GetSystem)))
    (:Is%20Not%20Valid
      (bind _returnvalue (SaveGame|DoesSaveGameExist (CallFunction|GetSystemSaveName)))
      (if _returnvalue
        (bind _returnvalue_2 (SaveGame|LoadGamefromSlot (CallFunction|GetSystemSaveName)))
        (bind _assystem_save (Utilities|Casting|CastToSystem_Save _returnvalue_2)
          (:then
            (Variables|Default|SetSystem _assystem_save))
          (:CastFailed
            _))
        (else
          (bind _returnvalue_3 (SaveGame|CreateSaveGameObject "/Game/OpeyeIIContent/Core/Data/System_Save.System_Save_C"))
          (Variables|Default|SetSystem _returnvalue_3)))
      (return (Variables|Default|GetSystem)))))

(fn GetTarget
  (return 0))
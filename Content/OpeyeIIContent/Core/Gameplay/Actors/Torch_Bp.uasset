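; Torch actor that follows the player's eye gaze, in both live tracking and replay.
; On BeginPlay it casts player controller 0 to the eye tracker controller, falling back to the replayer controller and flagging replay mode.
; Each tick it moves to the active controller's gaze origin and sets its rotation so its X axis points opposite the gaze direction.
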(event EventBeginPlay
  (bind _returnvalue (Game|GetPlayerController 0))
  (bind _aseye_tracker_ctr (Utilities|Casting|CastToEyeTracker_Ctr _returnvalue)
    (:then
      (Variables|Default|SetEyeTracker _aseye_tracker_ctr))
    (:CastFailed
      (Variables|Default|SetisReplaying true)
      (bind _aseye_tracker_replayer_ctr (Utilities|Casting|CastToEyeTrackerReplayer_Ctr _returnvalue))
      (Variables|Default|SetEyeTrackerReplay _aseye_tracker_replayer_ctr))))

(event EventTick
  (params (DeltaSeconds :type Float%20%28single-precision%29))
  (bind _eyetracker (Variables|Default|GetEyeTracker))
  (bind _eyetrackerreplay (Variables|Default|GetEyeTrackerReplay))
  (bind (_worldlocation _worlddirection) (Default|GetGazeOriginandDirection _eyetrackerreplay))
  (bind (_worldlocation_2 _worlddirection_2) (Default|GetGazeOriginandDirection _eyetracker))
  (if (Variables|Default|GetisReplaying)
    (Transformation|SetActorLocation _worldlocation false false)
    (Transformation|SetActorRotation (Math|Conversions|RotationFromXVector (* _worlddirection -1)))
    (else
      (Transformation|SetActorLocation _worldlocation_2 false false)
      (Transformation|SetActorRotation (Math|Conversions|RotationFromXVector (* _worlddirection_2 -1))))))

(fn ConstructionScript)
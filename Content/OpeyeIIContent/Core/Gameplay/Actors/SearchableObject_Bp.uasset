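; Searchable object actor for an eye-tracking visual search exercise, showing one mesh from a list as either the target or a distractor.
; Target setters update the Inspector pawn's search hint with the mesh name, while distractors pick random meshes intended to differ from it.
; Hits go through HitManagerCmp; when gaze tracking starts on the target, it saves all objects' mesh IDs to the pawn, plays the mesh's sound and calls the game mode's RetryMessage.
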(event Custom|EyesightIsTrackingMeAgain
  (bind _sounds (Variables|Default|GetSounds))
  (bind _currentmesh_id (Variables|Default|GetcurrentMesh_Id))
  (bind _output (Utilities|Array|Get(acopy) _sounds _currentmesh_id))
  (if (Variables|Default|GetisTarget)
    (CallFunction|SaveMeshesandTarget)
    (Variables|Default|SetisTarget false)
    (if (and (Utilities|IsValid _output) (< _currentmesh_id (Utilities|Array|Length _sounds)))
      (Audio|PlaySound2D _output 1.0 1.0 0.0 0 0)
      (Utilities|FlowControl|Delay 1.0))
    (Class|GameModeInt|Retry(Message) (Game|GetGameMode))))

(event Custom|ExerciseWasCompleted)

(event Custom|EyesightTrackWasLost)

(event Custom|EyetrackWasFullyLost)

(event Custom|SelectRandomAppearance
  (params (discardIndex :type Static%20Mesh%20Object%20Reference))
  (bind _meshes (Variables|Default|Getmeshes))
  (Variables|Default|SetcurrentMesh_Id (.OutIndex (Utilities|Array|Random _meshes)) :!label _label)
  (if (!= discardIndex (Utilities|Array|Get(acopy) _meshes (Variables|Default|GetcurrentMesh_Id)))
    (Components|StaticMesh|SetStaticMesh (Variables|Default|GetStaticMesh) (Utilities|Array|Get(acopy) _meshes (Variables|Default|GetcurrentMesh_Id)))
    (else
      (goto _label))))

(event Custom|ResetHit)

(event Custom|SetMeshID
  (params (id :type Integer))
  (Components|StaticMesh|SetStaticMesh (Variables|Default|GetStaticMesh) (Utilities|Array|Get(acopy) (Variables|Default|Getmeshes) id)))

(event EventBeginPlay
  (bind _hitmanager_cmp (Variables|Default|GetHitManager_Cmp))
  (EventDispatchers|BindEventtoTrackLossWarning _hitmanager_cmp (delegate Custom|EyesightTrackWasLost))
  (EventDispatchers|BindEventtoExerciseComplete _hitmanager_cmp (delegate Custom|ExerciseWasCompleted))
  (EventDispatchers|BindEventtoStartedBeingTracked _hitmanager_cmp (delegate Custom|EyesightIsTrackingMeAgain))
  (EventDispatchers|BindEventtoTrackFullyLostWarning _hitmanager_cmp (delegate Custom|EyetrackWasFullyLost)))

(event Collision|EventActorBeginOverlap
  (params (OtherActor :type Actor%20Object%20Reference)))

(event EventTick
  (params (DeltaSeconds :type Float%20%28single-precision%29)))

(event EventHit
  (params (Hit%20Component%20Name :type String))
  (Default|ManageHit (Variables|Default|GetHitManager_Cmp)))

(fn ConstructionScript
  (bind _meshes (Variables|Default|Getmeshes))
  (bind _returnvalue (Utilities|Array|Length _meshes))
  (if (> _returnvalue 0)
    (Components|StaticMesh|SetStaticMesh (Variables|Default|GetStaticMesh) (Utilities|Array|Get(acopy) _meshes (Math|Integer|Clamp(Integer) (Variables|Default|GetcurrentMesh_Id) 0 (- _returnvalue 1))))))

(fn GetStimulusObjectName
  (return (Utilities|String|Append "You hit: " (Utilities|GetObjectName (Utilities|Array|Get(acopy) (Variables|Default|Getmeshes) (Variables|Default|GetcurrentMesh_Id))))))

(fn SetasTarget
  (bind _meshes (Variables|Default|Getmeshes))
  (Variables|Default|SetisTarget true)
  (bind _output_get (Variables|Default|SetcurrentMesh_Id (Math|Random|RandomIntegerinRange 0 (- (Utilities|Array|Length _meshes) 1)) :!label _label))
  (Components|StaticMesh|SetStaticMesh (Variables|Default|GetStaticMesh) (Utilities|Array|Get(acopy) _meshes _output_get))
  (Utilities|IsValid (Utilities|Array|Get(acopy) _meshes _output_get)
    (:Is%20Valid
      (bind _outactors (Actor|GetAllActorsOfClass "/Game/OpeyeIIContent/Core/Gameplay/Pawn/Inspector_Pwn.Inspector_Pwn_C"))
      (Default|UpdateSearchHint (Utilities|Array|Get(acopy) _outactors) (Utilities|GetObjectName (Utilities|Array|Get(acopy) _meshes _output_get)))
      (CallFunction|ResetHit)
      (return (Utilities|Array|Get(acopy) _meshes _output_get)))
    (:Is%20Not%20Valid
      (goto _label))))

(fn SaveMeshesandTarget
  (bind _outactors (Actor|GetAllActorsOfClass "SearchableObject_Bp_C"))
  (bind _asinspector_pwn (Utilities|Casting|CastToInspector_Pwn (Game|Player|GetPlayerPawn 0)))
  (LocalVariables|SetInspectorPawn _asinspector_pwn)
  (for _array_element _outactors
    (bind _returnvalue (Utilities|Array|Add (LocalVariables|GetmeshesIds) (Variables|SearchableObject_Bp_C|GetcurrentMesh_Id _array_element)))
    (if (Variables|SearchableObject_Bp_C|GetisTarget _array_element)
      (bind _output_get (LocalVariables|SetwhichOneIsTarget _returnvalue))
      (Development|PrintString (Utilities|String|ToString(Integer) _output_get))))
  (Utilities|Array|Add (Variables|/Game/OpeyeIIContent/Core/Gameplay/Pawn/Inspector_Pwn.Inspector_Pwn_C|GetextraData (LocalVariables|GetInspectorPawn)) (Utilities|Struct|MakeSmoothPursuitD_ExtraData (LocalVariables|GetmeshesIds) (LocalVariables|GetwhichOneIsTarget))))

(fn SetasKnownTarget
  (Variables|Default|SetisTarget true)
  (bind _outactors (Actor|GetAllActorsOfClass "/Game/OpeyeIIContent/Core/Gameplay/Pawn/Inspector_Pwn.Inspector_Pwn_C"))
  (Default|UpdateSearchHint (Utilities|Array|Get(acopy) _outactors) (Utilities|GetObjectName (Variables|/Script/Engine.StaticMeshComponent|GetStaticMesh (Variables|Default|GetStaticMesh))))
  (CallFunction|ResetHit))

(fn GetTarget
  (return 0))
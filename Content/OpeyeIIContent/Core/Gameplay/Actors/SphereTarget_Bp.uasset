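; Sphere target actor for an eye-tracking exercise, colored through a dynamic material from the saved color scheme.
; Each tick it sweeps along the Y and Z components of a look direction toward the player, captured at BeginPlay, keeping X fixed.
; The first Hit always reports success to the Spline, adds the normalized mouse position as a seek location, destroys itself and resets spawning.
; Tracking-loss and completion handlers are bound but empty.
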(event Custom|EyesightIsTrackingMeAgain)

(event Custom|ExerciseWasCompleted)

(event Custom|EyesightTrackWasLost)

(event Custom|EyetrackWasFullyLost)

(event EventTick
  (params (DeltaSeconds :type Float%20%28single-precision%29))
  (bind _returnvalue (Transformation|GetActorLocation))
  (bind _look_rotation (Variables|Default|GetLook%20Rotation))
  (bind _speed (Variables|Default|GetSpeed))
  (bind _returnvalue_2 (Math|Vector|GetForwardVector _look_rotation))
  (bind _returnvalue_3 (* _returnvalue_2 _speed))
  (bind _returnvalue_4 (+ _returnvalue_3 _returnvalue))
  (bind (_x _y _z) (Math|Vector|BreakVector _returnvalue_4))
  (Transformation|SetActorLocation (Math|Vector|MakeVector (.X (Math|Vector|BreakVector _returnvalue)) _y _z) true false))

(event EventBeginPlay
  (bind _hitmanager_cmp (Variables|Default|GetHitManager_Cmp))
  (bind _lookrotation (CallFunction|GetLookRotation))
  (Variables|Default|SetLook%20Rotation _lookrotation)
  (EventDispatchers|BindEventtoTrackLossWarning _hitmanager_cmp (delegate Custom|EyesightTrackWasLost))
  (EventDispatchers|BindEventtoExerciseComplete _hitmanager_cmp (delegate Custom|ExerciseWasCompleted))
  (EventDispatchers|BindEventtoStartedBeingTracked _hitmanager_cmp (delegate Custom|EyesightIsTrackingMeAgain))
  (EventDispatchers|BindEventtoTrackFullyLostWarning _hitmanager_cmp (delegate Custom|EyetrackWasFullyLost)))

(event EventHit
  (params (Hit%20Component%20Name :type String))
  (bind _spline (Variables|Default|GetSpline))
  (Utilities|FlowControl|DoOnce false
    (:Completed
      (Default|ManageHit (Variables|Default|GetHitManager_Cmp))
      (bind _returnvalue (Class|WidgetLayoutLibrary|GetMousePositiononViewport))
      (Default|NotifyTargetResult _spline (Transformation|GetWorldLocation (Variables|Default|GetDefaultSceneRoot)) true) ; we always set it to yes here because in this exercise we do not judge how well a value is
      (Default|AddNewSeekLocation _spline (.As%20Vector%202D (CallFunction|GetNormalizedPositionOfEye _returnvalue)))
      (Actor|DestroyActor)
      (Default|ResetSpawn (Variables|Default|GetSpline)))))

(fn ConstructionScript
  (bind _systemsave (CallFunction|GetSystemSave))
  (bind _returnvalue (Rendering|Material|CreateDynamicMaterialInstance (Variables|Default|GetSphere) 0 "/Game/OpeyeIIContent/Art/Base/BaseMaterial.BaseMaterial" "None" :!class /Script/Engine.PrimitiveComponent))
  (Rendering|Material|SetVectorParameterValue _returnvalue "BaseColor" (Utilities|Select :Index (Variables|/Game/OpeyeIIContent/Core/Data/System_Save.System_Save_C|GetA_ColorConfig _systemsave) :NewEnumerator0 "(R=0.278894,G=1.000000,B=0.119538,A=1.000000)" :NewEnumerator1 "(R=1.000000,G=1.000000,B=1.000000,A=1.000000)" :NewEnumerator2 "(R=0.008568,G=0.127438,B=0.024158,A=1.000000)" :NewEnumerator3 "(R=0.913099,G=0.846873,B=0.000000,A=1.000000)" :NewEnumerator4 "(R=0.913099,G=0.846873,B=0.000000,A=1.000000)" :NewEnumerator5 "(R=1.000000,G=0.000000,B=0.000000,A=1.000000)" :NewEnumerator6 "(R=1.000000,G=1.000000,B=0.000000,A=1.000000)") :!class /Script/Engine.MaterialInstanceDynamic))

(fn GetLookRotation
  (return (Math|Rotator|FindLookatRotation (Transformation|GetActorLocation) (Transformation|GetActorLocation (Game|Player|GetPlayerPawn 0)))))

(fn GetNormalizedPositionOfEye
  (params (A :type Vector%202D%20Structure))
  (bind _returnvalue (Viewport|GetViewportSize))
  (bind _returnvalue_2 (Class|WidgetLayoutLibrary|GetViewportScale))
  (bind (_x _y) (Math|Vector2D|BreakVector2D _returnvalue))
  (bind _returnvalue_3 (* A _returnvalue_2))
  (bind (_x_2 _y_2) (Math|Vector2D|BreakVector2D _returnvalue_3))
  (bind _returnvalue_4 (/ _y 2.0))
  (bind _returnvalue_5 (/ _x 2.0))
  (bind _returnvalue_6 (- _x_2 _returnvalue_5))
  (bind _returnvalue_7 (- _y_2 _returnvalue_4))
  (bind _returnvalue_8 (/ _returnvalue_6 _returnvalue_5))
  (bind _returnvalue_9 (/ _returnvalue_7 _returnvalue_4))
  (return _returnvalue_8 _returnvalue_9 (Math|Vector2D|MakeVector2D _returnvalue_8 _returnvalue_9)))

(fn GetSystemSave
  (Utilities|IsValid (Variables|Default|GetSystem)
    (:Is%20Valid
      (return (Variables|Default|GetSystem)))
    (:Is%20Not%20Valid
      (bind _returnvalue (SaveGame|DoesSaveGameExist (CallFunction|GetSystemSaveName)))
      (if _returnvalue
        (bind _returnvalue_2 (SaveGame|LoadGamefromSlot (CallFunction|GetSystemSaveName)))
        (bind _assystem_save (Utilities|Casting|CastToSystem_Save _returnvalue_2)
          (:then
            (Variables|Default|SetSystem _assystem_save))
          (:CastFailed
            _))
        (else
          (bind _returnvalue_3 (SaveGame|CreateSaveGameObject "/Game/OpeyeIIContent/Core/Data/System_Save.System_Save_C"))
          (Variables|Default|SetSystem _returnvalue_3)))
      (return (Variables|Default|GetSystem)))))

(fn GetTarget
  (return 0))
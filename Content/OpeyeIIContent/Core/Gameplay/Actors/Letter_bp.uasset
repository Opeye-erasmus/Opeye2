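; Letter actor for a hit-based exercise in which a chain of letters is revealed one at a time.
; Hits go to HitManagerCmp, whose completion event reveals the active letter's text, notifies the Spawner and activates NextLetter with a highlight color.
; Tick accumulates time while the letter is active and unrevealed.
; Normal color and scale come from a cached System_Save, loaded or created on first use.
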(event Custom|SetActiveColor
  (bind _systemsave (CallFunction|GetSystemSave))
  (Rendering|Components|TextRender|SetTextRenderColor (Variables|Default|GetTextRender) (select (Utilities|Enum|NotEqual(Enum) (Variables|/Game/OpeyeIIContent/Core/Data/System_Save.System_Save_C|GetA_ColorConfig _systemsave) "NewEnumerator5") (Math|Conversions|ToColor(LinearColor) "(R=1.000000,G=0.000000,B=0.000000,A=1.000000)") (Math|Conversions|ToColor(LinearColor) "(R=1.000000,G=0.926360,B=0.000000,A=1.000000)")))
  (Variables|Default|SetisActive true))

(event Custom|ExerciseWasCompleted
  ;[1 1 1] Is letter active? If yes, it can do stuff
  (if (Variables|Default|GetisActive)
    ;[1 1 1] Has it been already revealed? If not, show
    (if (not (Variables|Default|GetisRevealed))
      (Default|CanEnd (Variables|Default|GetSpawner) (Variables|Default|GetletterIndex))
      ;[1 1 1] Set text to the letter it was assigned before
      (Rendering|Components|TextRender|SetText (Variables|Default|GetTextRender) (Variables|Default|GetLetter))
      (Class|ListenerInt|ListenedActorIsDone(Message) (Variables|Default|GetSpawner) self)
      ;[1 1 1] The current letter is revealed, and if there is a next one it can now be revealed by activating it
      (Variables|Default|SetisRevealed true)
      (bind _nextletter (Variables|Default|GetNextLetter)
        (:then
          (CallFunction|SetActiveColor _nextletter)
          (CallFunction|GetSaveSizeandColor))
        (:else)))))

(event EventBeginPlay
  (CallFunction|GetSaveSizeandColor)
  (EventDispatchers|BindEventtoExerciseComplete (Variables|Default|GetHitManager_Cmp) (delegate Custom|ExerciseWasCompleted)))

(event EventTick
  (params (DeltaSeconds :type Float%20%28single-precision%29))
  (if (Variables|Default|GetisActive)
    (if (not (Variables|Default|GetisRevealed))
      (Variables|Default|SettimeElapsed (+ DeltaSeconds (Variables|Default|GettimeElapsed))))))

(event EventHit
  (params (Hit%20Component%20Name :type String))
  (Default|ManageHit (Variables|Default|GetHitManager_Cmp)))

(fn ConstructionScript)

(fn GetSaveSizeandColor
  (bind _systemsave (CallFunction|GetSystemSave))
  (bind _output_get (LocalVariables|SetSave _systemsave))
  (Rendering|Components|TextRender|SetTextRenderColor (Variables|Default|GetTextRender) (Math|Conversions|ToColor(LinearColor) (Utilities|Select :Index (Variables|/Game/OpeyeIIContent/Core/Data/System_Save.System_Save_C|GetA_ColorConfig _output_get) :NewEnumerator0 "(R=0.278894,G=1.000000,B=0.119538,A=1.000000)" :NewEnumerator1 "(R=1.000000,G=1.000000,B=1.000000,A=1.000000)" :NewEnumerator2 "(R=0.008568,G=0.127438,B=0.024158,A=1.000000)" :NewEnumerator3 "(R=0.913099,G=0.846873,B=0.000000,A=1.000000)" :NewEnumerator4 "(R=0.913099,G=0.846873,B=0.000000,A=1.000000)" :NewEnumerator5 "(R=1.000000,G=0.000000,B=0.000000,A=1.000000)" :NewEnumerator6 "(R=1.000000,G=1.000000,B=0.000000,A=1.000000)")))
  (switch Utilities|FlowControl|Switch|SwitchonSizes_Enum (Variables|/Game/OpeyeIIContent/Core/Data/System_Save.System_Save_C|GetA_Size (LocalVariables|GetSave))
    (:NewEnumerator0
      (Transformation|SetActorScale3D "0.700000,0.700000,0.700000"))
    (:NewEnumerator1
      (Transformation|SetActorScale3D "0.900000,0.900000,0.900000"))
    (:NewEnumerator2
      (Transformation|SetActorScale3D "1.100000,1.100000,1.100000"))))

(fn GetSystemSave
  (Utilities|IsValid (Variables|Default|GetSystem)
    (:Is%20Valid
      (return (Variables|Default|GetSystem)))
    (:Is%20Not%20Valid
      (bind _returnvalue (SaveGame|DoesSaveGameExist (CallFunction|GetSystemSaveName)))
      (if _returnvalue
        (bind _returnvalue_2 (SaveGame|LoadGamefromSlot (CallFunction|GetSystemSaveName)))
        (bind _assystem_save (Utilities|Casting|CastToSystem_Save _returnvalue_2)
          (:then
            (Variables|Default|SetSystem _assystem_save))
          (:CastFailed
            _))
        (else
          (bind _returnvalue_3 (SaveGame|CreateSaveGameObject "/Game/OpeyeIIContent/Core/Data/System_Save.System_Save_C"))
          (Variables|Default|SetSystem _returnvalue_3)))
      (return (Variables|Default|GetSystem)))))

(fn GetTarget
  (return 0))
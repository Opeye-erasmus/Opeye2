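; Actor that destroys SphereTarget_Bp actors overlapping it, shown as a balloon-material sphere marked with a cross.
; On BeginPlay it builds a dynamic material, tinting the balloon from the color configuration in the system save.
; A hit asks Spline to spawn a target.
; An overlapping target increments a counter, resets the Spline's spawning and is destroyed.
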(event Collision|EventActorBeginOverlap
  (params (OtherActor :type Actor%20Object%20Reference))
  (bind _assphere_target_bp (Utilities|Casting|CastToSphereTarget_Bp OtherActor))
  (Math|Integer|IncrementInt (Variables|Default|GetCount)
    (:%20%20
      (Default|ResetSpawn (Variables|Default|GetSpline))
      (Actor|DestroyActor _assphere_target_bp))))

(event EventBeginPlay
  (bind _systemsave (CallFunction|GetSystemSave))
  (bind _returnvalue (Rendering|Material|CreateDynamicMaterialInstance (Variables|Default|GetSphere) 0 "/Game/OpeyeIIContent/Art/Props/Balloons/M_Balloon.M_Balloon" "None" :!class /Script/Engine.PrimitiveComponent))
  (Rendering|Material|SetTextureParameterValue _returnvalue "Object" "/Game/OpeyeIIContent/Art/Props/Shapes/cross.cross")
  (Rendering|Material|SetVectorParameterValue _returnvalue "BalloonColor" (Utilities|Select :Index (Variables|/Game/OpeyeIIContent/Core/Data/System_Save.System_Save_C|GetA_ColorConfig _systemsave) :NewEnumerator0 "(R=0.278894,G=1.000000,B=0.119538,A=1.000000)" :NewEnumerator1 "(R=1.000000,G=1.000000,B=1.000000,A=1.000000)" :NewEnumerator2 "(R=0.008568,G=0.127438,B=0.024158,A=1.000000)" :NewEnumerator3 "(R=0.913099,G=0.846873,B=0.000000,A=1.000000)" :NewEnumerator4 "(R=0.913099,G=0.846873,B=0.000000,A=1.000000)" :NewEnumerator5 "(R=1.000000,G=0.000000,B=0.000000,A=1.000000)" :NewEnumerator6 "(R=1.000000,G=1.000000,B=0.000000,A=1.000000)") :!class /Script/Engine.MaterialInstanceDynamic))

(event EventHit
  (params (Hit%20Component%20Name :type String))
  (Default|SpawnTarget (Variables|Default|GetSpline)))

(fn ConstructionScript)

(fn GetTarget
  (return 0))
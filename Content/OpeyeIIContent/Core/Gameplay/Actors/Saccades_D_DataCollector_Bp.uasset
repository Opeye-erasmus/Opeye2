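; Data collector for the saccades task that gathers timing results from letter and word actors when LoadData is called.
; It finds all Letter_bp and WordSpawner_Bp actors, storing each TimeElapsed in separate arrays and computing a mean per group.
; Both means are printed for debugging, but the printed values divide the already averaged time by the actor count a second time.
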(event Custom|LoadData
  (bind _outactors (Actor|GetAllActorsOfClass "/Game/OpeyeIIContent/Core/Gameplay/Actors/Letter_bp.Letter_bp_C"))
  (for _array_element _outactors
    (Variables|Default|SetmeanTimeLetters (+ (Variables|/Game/OpeyeIIContent/Core/Gameplay/Actors/Letter_bp.Letter_bp_C|GettimeElapsed _array_element) (Variables|Default|GetmeanTimeLetters)))
    (Utilities|Array|Add (Variables|Default|GettimeLetters) (Variables|/Game/OpeyeIIContent/Core/Gameplay/Actors/Letter_bp.Letter_bp_C|GettimeElapsed _array_element)))
  (Variables|Default|SetmeanTimeLetters (/ (Variables|Default|GetmeanTimeLetters) (Math|Conversions|ToFloat(Integer) (Utilities|Array|Length _outactors))))
  (Development|PrintString (Utilities|String|Append "Mean time letters: " (Utilities|String|ToString(Float) (/ (Variables|Default|GetmeanTimeLetters) (Math|Conversions|ToFloat(Integer) (Utilities|Array|Length _outactors))))))
  (bind _outactors_2 (Actor|GetAllActorsOfClass "/Game/OpeyeIIContent/Core/Gameplay/Spawners/WordSpawner_Bp.WordSpawner_Bp_C"))
  (for _array_element_2 _outactors_2
    (Variables|Default|SetmeanTimeWords (+ (Variables|/Game/OpeyeIIContent/Core/Gameplay/Spawners/WordSpawner_Bp.WordSpawner_Bp_C|GettimeElapsed _array_element_2) (Variables|Default|GetmeanTimeWords)))
    (Utilities|Array|Add (Variables|Default|GettimeWords) (Variables|/Game/OpeyeIIContent/Core/Gameplay/Spawners/WordSpawner_Bp.WordSpawner_Bp_C|GettimeElapsed _array_element_2)))
  (Variables|Default|SetmeanTimeWords (/ (Variables|Default|GetmeanTimeWords) (Math|Conversions|ToFloat(Integer) (Utilities|Array|Length _outactors_2))))
  (Development|PrintString (Utilities|String|Append "Mean time words: " (Utilities|String|ToString(Float) (/ (Variables|Default|GetmeanTimeWords) (Math|Conversions|ToFloat(Integer) (Utilities|Array|Length _outactors_2)))))))

(fn ConstructionScript)
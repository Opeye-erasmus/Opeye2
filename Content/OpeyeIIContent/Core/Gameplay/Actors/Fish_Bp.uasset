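; Fish actor for an eye-gaze game that swims along a diving spline until the player's gaze holds it still.
; Hits stop its swim timeline; it resumes half a second after the last one.
; If left unspotted past a speed-scaled timeout, it plays a jump-spline timeline, then triggers the pawn's game-over message.
; Swim speed comes from the system save, while DataCollector records speed, unspotted times and laps.
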(event Custom|MoveFish
  (bind _divingpath_spline (Variables|Default|GetDivingPath_Spline))
  (Components|Timeline|SetPlayRate (Variables|Default|GetMoveTimeline) (/ (Variables|Default|GetSpeenSpeed) (Variables|Default|GetLoopRate)))
  (if (== (Components|Timeline|GetPlaybackPosition (Variables|Default|GetMoveTimeline)) 0.0)
    (bind _distance (Timeline|MoveTimeline ReverseFromEnd)
      (:Update
        (Transformation|SetRelativeTransform (Variables|Default|GetStaticMesh) (Math|Transform|MakeTransform (Spline|GetLocationatDistanceAlongSpline _divingpath_spline (Math|Float|Lerp 0.0 (Spline|GetSplineLength _divingpath_spline) _distance) "Local") (Spline|GetRotationatDistanceAlongSpline _divingpath_spline (Math|Float|Lerp 0.0 (Spline|GetSplineLength _divingpath_spline) _distance) "Local") (Variables|Default|GetFishScale)) false false))
      (:Finished
        (bind _result (Math|Integer|IncrementInt (Variables|/Game/OpeyeIIContent/Core/Gameplay/Actors/Saccades_B_DataCollector_Bp.Saccades_B_DataCollector_Bp_C|Getlaps (Variables|Default|GetdataCollector))))))
    (else
      (Timeline|MoveTimeline Reverse))))

(event Custom|Jump
  (bind _jumpingpath_spline (Variables|Default|GetJumpingPath_Spline))
  (Components|Timeline|SetPlayRate (Variables|Default|GetTimeline_Jump) (/ 1.0 (Variables|Default|GetLoopRate)))
  (bind _distance (Timeline|Timeline_Jump ReverseFromEnd)
    (:Update
      (Transformation|SetRelativeTransform (Variables|Default|GetStaticMesh) (Math|Transform|MakeTransform (Spline|GetLocationatDistanceAlongSpline _jumpingpath_spline (Math|Float|Lerp 0.0 (Spline|GetSplineLength _jumpingpath_spline) _distance) "Local") (Spline|GetRotationatDistanceAlongSpline _jumpingpath_spline (Math|Float|Lerp 0.0 (Spline|GetSplineLength _jumpingpath_spline) _distance) "Local") (Variables|Default|GetFishScale)) false false))
    (:Finished
      (Class|PlayerInt|GameIsOver(Message) (Game|Player|GetPlayerPawn 0)))))

(event EventBeginPlay
  (Variables|Default|SetFishScale (Variables|/Script/Engine.SceneComponent|GetRelativeScale3D (Variables|Default|GetStaticMesh)))
  (Variables|Default|SetlastTimeBeingSpotted (Math|DateTime|Now))
  (bind _outactors (Actor|GetAllActorsOfClass "/Game/OpeyeIIContent/Core/Gameplay/Pawn/Saccade_Pwn.Saccade_Pwn_C"))
  (if (Variables|/Game/OpeyeIIContent/Core/Gameplay/Pawn/Saccade_Pwn.Saccade_Pwn_C|GetbTick (Utilities|Array|Get(acopy) _outactors))
    (bind _newparam (CallFunction|GetSystemSave))
    (bind _output_get (Variables|/Game/OpeyeIIContent/Core/Gameplay/Actors/Saccades_B_DataCollector_Bp.Saccades_B_DataCollector_Bp_C|Setspeed (Variables|Default|GetdataCollector) (Variables|/Game/OpeyeIIContent/Core/Data/System_Save.System_Save_C|GetA_Speed _newparam)))
    (switch Utilities|FlowControl|Switch|SwitchonSaccades_Speed_Enum _output_get
      (:NewEnumerator0
        (Variables|Default|SetSpeenSpeed 0.5))
      (:NewEnumerator1
        (Variables|Default|SetSpeenSpeed 1.0))
      (:NewEnumerator2
        (Variables|Default|SetSpeenSpeed 1.5)))))

(event EventTick
  (params (DeltaSeconds :type Float%20%28single-precision%29))
  (bind _returnvalue (Math|DateTime|Now))
  (bind _lasttimebeingspotted (Variables|Default|GetlastTimeBeingSpotted))
  (bind _returnvalue_2 (- _returnvalue _lasttimebeingspotted))
  (bind _returnvalue_3 (Math|Timespan|GetTotalSeconds _returnvalue_2))
  (Utilities|FlowControl|Delay 0.2)
  (if (not (Variables|Default|GetisBeingStared))
    (Default|SaveTimeLeap (Variables|Default|GetdataCollector) _returnvalue_3)
    (if (> _returnvalue_3 (/ (Variables|Default|GetJumpTimeout) (Variables|Default|GetSpeenSpeed)))
      (Utilities|FlowControl|DoOnce false
        (:Completed
          (CallFunction|Jump)))
      (elif (== (Components|Timeline|GetPlaybackPosition (Variables|Default|GetMoveTimeline)) 0.0)
        (CallFunction|MoveFish :!label _label)))
    (elif (> (Math|Timespan|GetTotalSeconds (- (Math|DateTime|Now) (Variables|Default|GetlastTimeBeingSpotted))) 0.5)
      (CallFunction|BeingIgnored)
      (goto _label))))

(event EventHit
  (params (Hit%20Component%20Name :type String))
  (bind _outactors (Actor|GetAllActorsOfClass "Fish_Bp_C"))
  (for _array_element _outactors
    (if (== _array_element self)
      (CallFunction|ReceiveEyeSight _array_element))))

(fn ConstructionScript)

(fn ReceiveEyeSight
  (Variables|Default|SetisBeingStared true)
  (Variables|Default|SetlastTimeBeingSpotted (Math|DateTime|Now))
  (Audio|Components|Audio|Stop (Variables|Default|GetMoveTimeline)))

(fn BeingIgnored
  (Variables|Default|SetisBeingStared false))

(fn GetSystemSave
  (Utilities|IsValid (Variables|Default|GetSystem)
    (:Is%20Valid
      (return (Variables|Default|GetSystem)))
    (:Is%20Not%20Valid
      (bind _returnvalue (SaveGame|DoesSaveGameExist (CallFunction|GetSystemSaveName)))
      (if _returnvalue
        (bind _returnvalue_2 (SaveGame|LoadGamefromSlot (CallFunction|GetSystemSaveName)))
        (bind _assystem_save (Utilities|Casting|CastToSystem_Save _returnvalue_2)
          (:then
            (Variables|Default|SetSystem _assystem_save))
          (:CastFailed
            _))
        (else
          (bind _returnvalue_3 (SaveGame|CreateSaveGameObject "/Game/OpeyeIIContent/Core/Data/System_Save.System_Save_C"))
          (Variables|Default|SetSystem _returnvalue_3)))
      (return (Variables|Default|GetSystem)))))

(fn GetJitteringComponent
  (return 0))

(fn GetTarget
  (return 0))
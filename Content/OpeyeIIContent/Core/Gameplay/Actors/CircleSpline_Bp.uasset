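; CircleSpline_Bp is a training actor that spawns sphere targets one at a time along a spline, scaled by the saved dot size.
; In training, BeginPlay shuffles evenly spaced spline distances, which a resettable DoOnce gate consumes per SpawnTarget call.
; Reported hits and misses become blue or red result spheres after the last target, then FOV_Pwn is notified following a delay.
; In replay, it only loads the dot size.
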(event Custom|SpawnTarget
  ;[1 1 1] Spawn target along a distance in the spline
  (Utilities|FlowControl|DoOnce false
    (:Completed
      (if (< (Variables|Default|Getindex) (Variables|Default|GetmaxObjectsToSpawn))
        (bind _returnvalue (Game|SpawnActorfromClass "/Game/OpeyeIIContent/Core/Gameplay/Actors/SphereTarget_Bp.SphereTarget_Bp_C" (Math|Transform|MakeTransform (Spline|GetLocationatDistanceAlongSpline (Variables|Default|GetSpline) (Utilities|Array|Get(acopy) (Variables|Default|Getdistances) (Variables|Default|Getindex)) "World") "0, 0, 0" (* "1.000000,1.000000,1.000000" (Utilities|Select :Index (Variables|Default|GetDotsSize) :NewEnumerator0 0.5 :NewEnumerator1 1.0 :NewEnumerator2 1.5))) "Undefined" 0 0 0))
        (Variables|/Game/OpeyeIIContent/Core/Gameplay/Actors/SphereTarget_Bp.SphereTarget_Bp_C|SetSpline _returnvalue self)
        (Math|Integer|IncrementInt (Variables|Default|Getindex))
        (else
          ;[1 1 1] Show results at the end
          (for _array_element (Variables|Default|GetReport)
            (bind _returnvalue_2 (Game|SpawnActorfromClass "/Game/OpeyeIIContent/Core/Gameplay/Actors/SphereTargetResult_Bp.SphereTargetResult_Bp_C" (Math|Transform|MakeTransform (.FinalLocation (Utilities|Struct|BreakTargetResultInfo_Str _array_element)) "0, 0, 0" "0.300000,0.300000,0.300000") "Undefined" 0 0))
            (Default|SetMaterial _returnvalue_2 (select (.Success (Utilities|Struct|BreakTargetResultInfo_Str _array_element)) "/Game/OpeyeIIContent/Art/Props/Wardrobe/clothes/Res/Blue_Mat.Blue_Mat" "/Game/OpeyeIIContent/Art/Props/Wardrobe/clothes/Res/Red_Mat.Red_Mat")))
          (Utilities|FlowControl|Delay 3.0)
          (bind _asfov_pwn (Utilities|Casting|CastToFOV_Pwn (Game|Player|GetPlayerPawn 0)))
          (Default|ListenedActorIsDone _asfov_pwn))))))

(event Custom|ResetSpawn
  ;[1 1 1] Spawn target along a distance in the spline
  (Utilities|FlowControl|DoOnce false) ; enters at Reset
)

(event Custom|NotifyTargetResult
  (params (Location :type Vector) (Success :type Boolean))
  (Utilities|Array|Add (Variables|Default|GetReport) (Utilities|Struct|MakeTargetResultInfo_Str Location Success)))

(event EventBeginPlay
  (Utilities|Casting|CastToFOV_Pwn (Game|Player|GetPlayerPawn 0)
    (:then
      ;[1 1 1] training
      (bind _systemsave (CallFunction|GetSystemSave))
      (Variables|Default|Setindex 0)
      (Variables|Default|SetDotsSize (Variables|/Game/OpeyeIIContent/Core/Data/System_Save.System_Save_C|GetA_Size _systemsave))
      (Variables|Default|SetmaxObjectsToSpawn 20)
      (CallFunction|CalculateAddedDistance)
      (CallFunction|CreateDistanceArrayandShuffle))
    (:CastFailed
      ;[1 1 1] Replay
      (bind _systemsave_2 (CallFunction|GetSystemSave))
      (Variables|Default|SetDotsSize (Variables|/Game/OpeyeIIContent/Core/Data/System_Save.System_Save_C|GetA_Size _systemsave_2)))))

(fn ConstructionScript)

(fn AddNewSeekLocation
  (params (seekLocation :type Vector%202D%20Structure))
  (Utilities|Array|Add (Variables|Default|GeteyeSeekLocations) seekLocation)
  (Utilities|FlowControl|Sequence
    (:then_0
      (if (> (Math|Float|Absolute(Float) (Math|Vector|Distance2D(Vector) :V2 seekLocation)) (Math|Float|Absolute(Float) (Math|Vector|Distance2D(Vector) "(X=0.000000,Y=0.000000)" (Variables|Default|GetfarthestLocation))))
        (Variables|Default|SetfarthestLocation seekLocation)))
    (:then_1
      (if (< (Math|Float|Absolute(Float) (Math|Vector|Distance2D(Vector) :V2 seekLocation)) (Math|Float|Absolute(Float) (Math|Vector|Distance2D(Vector) :V2 (Variables|Default|GetnearestLocation))))
        (Variables|Default|SetnearestLocation seekLocation)))))

(fn CalculateAddedDistance
  (Variables|Default|SetaddedDistance (/ (Spline|GetSplineLength (Variables|Default|GetSpline)) (Math|Conversions|ToFloat(Integer) (+ (Variables|Default|GetmaxObjectsToSpawn) 1)))))

(fn CreateDistanceArrayandShuffle
  (for _index (range 0 (Variables|Default|GetmaxObjectsToSpawn))
    (Utilities|Array|Add (Variables|Default|Getdistances) (* _index (Variables|Default|GetaddedDistance)))
    (Development|PrintString (Utilities|String|ToString(Float) (* _index (Variables|Default|GetaddedDistance)))))
  (Utilities|Array|Shuffle (Variables|Default|Getdistances)))

(fn GetTargetReport
  (return (Variables|Default|GetReport)))
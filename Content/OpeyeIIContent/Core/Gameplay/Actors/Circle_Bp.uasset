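; Gaze-tracked moving circle with a balloon material, which travels between Target_Bp actors in a smooth-pursuit eye exercise and totals time seen and unseen.
; HitManagerCmp reports gaze tracking, which sets the initial target (Id -1) and starts travel.
; Interface-found components handle movement and next-target strategy, keeping both swappable.
; Target Ids are recorded under SmoothPursuit_Pwn and fed to SelectNextTarget4AxesCmp for replays.
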(event OnPrimitiveLostGazeFocus(TobiiGazeFocusable)
  (params (FocusedComponent :type Primitive%20Component%20Object%20Reference)))

(event OnPrimitiveReceivedGazeFocus(TobiiGazeFocusable)
  (params (FocusedComponent :type Primitive%20Component%20Object%20Reference)))

(event Custom|EyesightIsTrackingMeAgain
  (bind _returnvalue (Class|Actor|GetComponentsbyInterface "/Game/OpeyeIIContent/Core/Gameplay/Interfaces/TravelerComponent_Int.TravelerComponent_Int_C"))
  (if (> (Utilities|Array|Length _returnvalue) 0)
    (CallFunction|FindInitialTarget)
    (Class|TravelerComponentInt|Start(Message) (Utilities|Array|Get(acopy) _returnvalue))
    (else
      (CallFunction|FindInitialTarget)
      (Class|TravelerComponentInt|Start(Message) (Variables|Default|GetCurrentTarget)))))

(event Custom|Start
  (params (directions :type Directions_Enum%20Enum :default "NewEnumerator0"))
  (bind _returnvalue (Class|Actor|GetComponentsbyInterface "/Game/OpeyeIIContent/Core/Gameplay/Interfaces/FindTargetStrategy_Int.FindTargetStrategy_Int_C"))
  (bind _output (Utilities|Array|Get(acopy) _returnvalue))
  (if (> (Utilities|Array|Length _returnvalue) 0)
    (Class|FindTargetStrategyInt|SetMode(Message) _output directions)
    (bind _target (Class|FindTargetStrategyInt|ResetPosition(Message) _output))
    (Variables|Default|SetCurrentTarget _target)))

(event Custom|LostTrack
  (Variables|Default|SetisSeen false))

(event Custom|SetReplayTargets
  (Variables|/Game/OpeyeIIContent/Core/Gameplay/Components/SelectNextTarget_4Axes_Cmp.SelectNextTarget_4Axes_Cmp_C|Settargets (Variables|Default|GetSelectNextTarget_4Axes_Cmp) (Variables|Default|Gettargets)))

(event Custom|SetMaterialColour
  (params (Value :type Linear%20Color%20Structure) (Object :type Texture%20Object%20Reference))
  (bind _staticmesh (Variables|Default|GetStaticMesh))
  (bind _returnvalue (Rendering|Material|CreateDynamicMaterialInstance _staticmesh 0 "/Game/OpeyeIIContent/Art/Props/Balloons/M_Balloon.M_Balloon" "None" :!class /Script/Engine.PrimitiveComponent))
  (Rendering|Material|SetVectorParameterValue _returnvalue "BalloonColor" Value :!class /Script/Engine.MaterialInstanceDynamic)
  (Rendering|Material|SetTextureParameterValue _returnvalue "Object" Object)
  (Rendering|Material|SetScalarParameterValueonMaterials _staticmesh "EmissiveInt" 1.0))

(event EventHit
  (params (Hit%20Component%20Name :type String))
  (Default|ManageHit (Variables|Default|GetHitManager_Cmp))
  (Variables|Default|SetisSeen true))

(event EventBeginPlay
  (bind _hitmanager_cmp (Variables|Default|GetHitManager_Cmp))
  (EventDispatchers|BindEventtoTrackFullyLostWarning _hitmanager_cmp (delegate Custom|LostTrack))
  (EventDispatchers|BindEventtoStartedBeingTracked _hitmanager_cmp (delegate Custom|EyesightIsTrackingMeAgain))
  (Default|Pause (Variables|Default|GetTravelToTarget_Cmp)))

(event EventTick
  (params (DeltaSeconds :type Float%20%28single-precision%29))
  (if (Variables|Default|GetisSeen)
    (Variables|Default|SettimeSeen (+ (Variables|Default|GettimeSeen) DeltaSeconds))
    (else
      (Variables|Default|SettimeNotSeen (+ DeltaSeconds (Variables|Default|GettimeNotSeen))))))

(event EventReachedTarget
  (bind _returnvalue (Class|Actor|GetComponentsbyInterface "/Game/OpeyeIIContent/Core/Gameplay/Interfaces/FindTargetStrategy_Int.FindTargetStrategy_Int_C"))
  (if (> (Utilities|Array|Length _returnvalue) 0)
    (bind _target (Class|FindTargetStrategyInt|Find(Message) (Utilities|Array|Get(acopy) _returnvalue)))
    (bind _output_get (Variables|Default|SetCurrentTarget _target))
    (bind _astarget_bp (Utilities|Casting|CastToTarget_Bp _output_get))
    ;[1 1 1] To detect we are not in a replay and therefore we are not editing the targets
    (Utilities|Casting|CastToSmoothPursuit_Pwn (Game|Player|GetPlayerPawn 0))
    (Utilities|Array|Add (Variables|Default|Gettargets) (Variables|/Game/OpeyeIIContent/Core/Gameplay/Actors/Target_Bp.Target_Bp_C|GetId _astarget_bp))))

(event EventSetTarget
  (params (target :type Actor%20Object%20Reference))
  (bind _returnvalue (Class|Actor|GetComponentsbyInterface "/Game/OpeyeIIContent/Core/Gameplay/Interfaces/TravelerComponent_Int.TravelerComponent_Int_C"))
  (Variables|Default|SetCurrentTarget target)
  (if (> (Utilities|Array|Length _returnvalue) 0)
    (Class|TravelerComponentInt|Start(Message) (Utilities|Array|Get(acopy) _returnvalue))))

(fn ConstructionScript)

(fn FindInitialTarget
  (bind _outactors (Actor|GetAllActorsOfClass "/Game/OpeyeIIContent/Core/Gameplay/Actors/Target_Bp.Target_Bp_C"))
  (bind _array_element (Utilities|Array|ForEachLoopwithBreak _outactors :!label _label)
    (:LoopBody
      (if (== (Variables|/Game/OpeyeIIContent/Core/Gameplay/Actors/Target_Bp.Target_Bp_C|GetId _array_element) -1)
        (bind _output_get (Variables|Default|SetCurrentTarget _array_element))
        (Utilities|Casting|CastToSmoothPursuit_Pwn (Game|Player|GetPlayerPawn 0))
        (bind _astarget_bp (Utilities|Casting|CastToTarget_Bp _output_get))
        (Utilities|Array|Add (Variables|Default|Gettargets) (Variables|/Game/OpeyeIIContent/Core/Gameplay/Actors/Target_Bp.Target_Bp_C|GetId _astarget_bp))
        (goto _label Break)))))

(fn GetJitteringComponent
  (return (Variables|Default|GetStaticMesh)))

(fn GetTarget
  (return (Variables|Default|GetCurrentTarget)))
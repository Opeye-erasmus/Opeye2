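; Eye-tracked balloon actor for the smooth pursuit exercise, skinned by colour and shape through a dynamic material.
; HitManagerCmp turns gaze hits into tracking events that resume travel, send it back to the origin Target_Bp, or end the game with a smiley.
; A pluggable strategy component picks each target and logs its ID, which replay mode follows instead.
; Tick accumulates seen and unseen time.
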(event OnPrimitiveReceivedGazeFocus(TobiiGazeFocusable)
  (params (FocusedComponent :type Primitive%20Component%20Object%20Reference))
  (Development|PrintString "Detefcted"))

(event Custom|EyesightIsTrackingMeAgain
  (bind _returnvalue (Class|Actor|GetComponentsbyInterface "/Game/OpeyeIIContent/Core/Gameplay/Interfaces/TravelerComponent_Int.TravelerComponent_Int_C"))
  (if (> (Utilities|Array|Length _returnvalue) 0)
    (CallFunction|FindTarget)
    (Class|TravelerComponentInt|Start(Message) (Utilities|Array|Get(acopy) _returnvalue))
    (else
      (CallFunction|FindTarget)
      (Class|TravelerComponentInt|Start(Message) (Variables|Default|GetCurrentTarget)))))

(event Custom|ExerciseWasCompleted
  ;[1 1 1] When user completes the exercise, show smiley and end game after 3 seconds
  (if (not (Variables|Default|GetisReplaying))
    (Game|SpawnActorfromClass "/Game/OpeyeIIContent/Core/Gameplay/Actors/Smiley_Bp.Smiley_Bp_C" (Math|Transform|MakeTransform "0,-200.000000,170.000000") "Undefined" 0 0)
    (Utilities|FlowControl|Delay 3.0)
    (bind _assmooth_pursuit_pwn (Utilities|Casting|CastToSmoothPursuit_Pwn (Game|Player|GetPlayerPawn 0)))
    (Default|EndGame _assmooth_pursuit_pwn)))

(event Custom|EyesightTrackWasLost)

(event Custom|EyetrackWasFullyLost
  (Variables|Default|SetisSeen false)
  (bind _outactors (Actor|GetAllActorsOfClass "/Game/OpeyeIIContent/Core/Gameplay/Actors/Target_Bp.Target_Bp_C"))
  (bind _array_element (Utilities|Array|ForEachLoopwithBreak _outactors :!label _label)
    (:LoopBody
      (if (== (Variables|/Game/OpeyeIIContent/Core/Gameplay/Actors/Target_Bp.Target_Bp_C|GetId _array_element) -1)
        (CallFunction|SetTarget _array_element)
        (goto _label Break)))))

(event Custom|SetMaterialColour
  (params (Colour :type Config_NewAvailableColours%20Enum :default "NewEnumerator0") (Shape :type Shapes_Enum%20Enum :default "NewEnumerator0"))
  (Rendering|SetActorHiddenInGame false)
  (bind _returnvalue (Rendering|Material|CreateDynamicMaterialInstance (Variables|Default|GetStaticMesh) 0 "/Game/OpeyeIIContent/Art/Props/Balloons/M_Balloon.M_Balloon" "None" :!class /Script/Engine.PrimitiveComponent))
  (Rendering|Material|SetVectorParameterValue _returnvalue "BalloonColor" (Utilities|Select :Index Colour :NewEnumerator0 "(R=0.278894,G=1.000000,B=0.119538,A=1.000000)" :NewEnumerator1 "(R=1.000000,G=1.000000,B=1.000000,A=1.000000)" :NewEnumerator2 "(R=0.008568,G=0.127438,B=0.024158,A=1.000000)" :NewEnumerator3 "(R=0.913099,G=0.846873,B=0.000000,A=1.000000)" :NewEnumerator4 "(R=0.913099,G=0.846873,B=0.000000,A=1.000000)" :NewEnumerator5 "(R=1.000000,G=0.000000,B=0.000000,A=1.000000)" :NewEnumerator6 "(R=1.000000,G=1.000000,B=0.000000,A=1.000000)") :!class /Script/Engine.MaterialInstanceDynamic)
  (Rendering|Material|SetTextureParameterValue _returnvalue "Object" (Utilities|Select :Index Shape :NewEnumerator0 "/Game/OpeyeIIContent/Art/Props/Shapes/circle.circle" :NewEnumerator1 "/Game/OpeyeIIContent/Art/Props/Shapes/square.square" :NewEnumerator2 "/Game/OpeyeIIContent/Art/Props/Shapes/smiley.smiley" :NewEnumerator3 "/Game/OpeyeIIContent/Art/Props/Shapes/apple.apple" :NewEnumerator4 "/Game/OpeyeIIContent/Art/Props/Shapes/house.house" :NewEnumerator5 "/Game/OpeyeIIContent/Art/Props/Balloons/Opeye_Balloon_Base.Opeye_Balloon_Base" :NewEnumerator6 "/Game/OpeyeIIContent/Art/Props/Shapes/bird.bird" :NewEnumerator7 "/Game/OpeyeIIContent/Art/Props/Shapes/kite.kite" :NewEnumerator8 "/Game/OpeyeIIContent/Art/Props/Shapes/bear.bear"))
  (Rendering|Material|SetScalarParameterValue _returnvalue "EmissiveInt" 1.0 :!class /Script/Engine.MaterialInstanceDynamic)
  (Rendering|SetVisibility (Variables|Default|GetKiteAddons) (Utilities|Enum|Equal(Enum) Shape "NewEnumerator7") false)
  (Rendering|SetVisibility (Variables|Default|GetBallonAddons) (Utilities|Enum|Equal(Enum) Shape "NewEnumerator5") false))

(event EventBeginPlay
  (bind _hitmanager_cmp (Variables|Default|GetHitManager_Cmp))
  (Default|Pause (Variables|Default|GetTravelToTarget_Cmp))
  (Utilities|FlowControl|Sequence
    (:then_2
      (EventDispatchers|BindEventtoTrackLossWarning _hitmanager_cmp (delegate Custom|EyesightTrackWasLost))
      (EventDispatchers|BindEventtoExerciseComplete _hitmanager_cmp (delegate Custom|ExerciseWasCompleted))
      (EventDispatchers|BindEventtoStartedBeingTracked _hitmanager_cmp (delegate Custom|EyesightIsTrackingMeAgain))
      (EventDispatchers|BindEventtoTrackFullyLostWarning _hitmanager_cmp (delegate Custom|EyetrackWasFullyLost)))))

(event EventTick
  (params (DeltaSeconds :type Float%20%28single-precision%29))
  (if (Variables|Default|GetisSeen)
    (Variables|Default|SettimeSeen (+ (Variables|Default|GettimeSeen) DeltaSeconds))
    (else
      (Variables|Default|SettimeNotSeen (+ DeltaSeconds (Variables|Default|GettimeNotSeen))))))

(event EventReachedTarget
  (bind _astarget_bp (Utilities|Casting|CastToTarget_Bp (Variables|Default|GetCurrentTarget)))
  (if (!= (Variables|/Game/OpeyeIIContent/Core/Gameplay/Actors/Target_Bp.Target_Bp_C|GetId _astarget_bp) -1)
    _
    (else
      (Default|Pause (Variables|Default|GetTravelToTarget_Cmp))))
  (CallFunction|FindTarget))

(event EventSetTarget
  (params (target :type Actor%20Object%20Reference))
  (Variables|Default|SetCurrentTarget target))

(event EventHit
  (params (Hit%20Component%20Name :type String))
  (Default|ManageHit (Variables|Default|GetHitManager_Cmp))
  (Variables|Default|SetisSeen true))

(fn ConstructionScript
  (Rendering|SetActorHiddenInGame true))

(fn FindTarget
  (bind _returnvalue (Class|Actor|GetComponentsbyInterface "/Game/OpeyeIIContent/Core/Gameplay/Interfaces/FindTargetStrategy_Int.FindTargetStrategy_Int_C"))
  (if (Variables|Default|GetisReplaying)
    (if (not (== (Utilities|Array|Length (Variables|Default|Gettargets)) (Variables|Default|Getindex)))
      (bind _outactors (Actor|GetAllActorsOfClass "/Game/OpeyeIIContent/Core/Gameplay/Actors/Target_Bp.Target_Bp_C"))
      (bind _array_element (Utilities|Array|ForEachLoopwithBreak _outactors :!label _label)
        (:LoopBody
          (LocalVariables|SetTarget _array_element)
          (if (== (Utilities|Array|Get(acopy) (Variables|Default|Gettargets) (Variables|Default|Getindex)) (Variables|/Game/OpeyeIIContent/Core/Gameplay/Actors/Target_Bp.Target_Bp_C|GetId _array_element))
            (goto _label Break)))
        (:Completed
          (CallFunction|SetTarget (LocalVariables|GetTarget))
          (Math|Integer|IncrementInt (Variables|Default|Getindex)))))
    (elif (> (Utilities|Array|Length _returnvalue) 0)
      (bind _target (Class|FindTargetStrategyInt|Find(Message) (Utilities|Array|Get(acopy) _returnvalue)))
      (bind _astarget_bp (Utilities|Casting|CastToTarget_Bp _target))
      (Utilities|Array|Add (Variables|Default|Gettargets) (Variables|/Game/OpeyeIIContent/Core/Gameplay/Actors/Target_Bp.Target_Bp_C|GetId _astarget_bp))
      (CallFunction|SetTarget _target)
      (Development|PrintString (Utilities|String|ToString(Integer) (Variables|/Game/OpeyeIIContent/Core/Gameplay/Actors/Target_Bp.Target_Bp_C|GetId _astarget_bp))))))

(fn GetJitteringComponent
  (return 0))

(fn GetTarget
  (return (Variables|Default|GetCurrentTarget)))
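; Static gaze target for a saccade eye exercise, sized from the system save and showing its halo only while active.
; While active, it tallies center and halo hits, forwards them to HitManagerCmp and runs a countdown from the saved time.
; On completion it records good or bad by remaining time, and perfect, overshoot or undershoot by hit distribution, in DataCollector.
; It then deactivates and notifies its parent actor.
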(event Custom|EyesightIsTrackingMeAgain)

(event Custom|ExerciseWasCompleted
  (bind _datacollector (Variables|Default|GetdataCollector))
  (bind _datacollector_2 (Variables|Default|GetdataCollector))
  (bind _datacollector_3 (Variables|Default|GetdataCollector))
  (bind _datacollector_4 (Variables|Default|GetdataCollector))
  (bind _datacollector_5 (Variables|Default|GetdataCollector))
  (bind _badhits (Variables|/Game/OpeyeIIContent/Core/Gameplay/Actors/Saccades_A_StimulusDataCollector_Bp.Saccades_A_StimulusDataCollector_Bp_C|GetbadHits _datacollector_2))
  (bind _goodhits (Variables|/Game/OpeyeIIContent/Core/Gameplay/Actors/Saccades_A_StimulusDataCollector_Bp.Saccades_A_StimulusDataCollector_Bp_C|GetgoodHits _datacollector))
  (bind _undershoots (Variables|/Game/OpeyeIIContent/Core/Gameplay/Actors/Saccades_A_StimulusDataCollector_Bp.Saccades_A_StimulusDataCollector_Bp_C|GetunderShoots _datacollector_4))
  (bind _overshoots (Variables|/Game/OpeyeIIContent/Core/Gameplay/Actors/Saccades_A_StimulusDataCollector_Bp.Saccades_A_StimulusDataCollector_Bp_C|GetoverShoots _datacollector_5))
  (bind _perfect (Variables|/Game/OpeyeIIContent/Core/Gameplay/Actors/Saccades_A_StimulusDataCollector_Bp.Saccades_A_StimulusDataCollector_Bp_C|Getperfect _datacollector_3))
  (CallFunction|DisableActiveMode)
  (Utilities|FlowControl|DoOnce true
    (:Completed
      ;[1 1 1] Check time against max time to track, good or bad
      (Math|Integer|IncrementInt (Variables|Default|GetnumberOfHits)
        (:%20%20
          (if (<= (Variables|Default|GetCount) 0)
            (Math|Integer|IncrementInt _badhits
              (:%20%20
                _))
            (else
              (Math|Integer|IncrementInt _goodhits
                (:%20%20
                  _))))
          (Development|PrintString (Utilities|String|Append "Bad Hits: " (Utilities|String|ToString(Integer) _badhits) " Good Hits: " (Utilities|String|ToString(Integer) _goodhits) " Count: " (Utilities|String|ToString(Integer) (Variables|Default|GetCount))))
          ;[1 1 1] More at center? Good hit
          (if (> (Variables|Default|GetcenterHits) (Variables|Default|GethaloHits))
            (Math|Integer|IncrementInt _perfect
              (:%20%20
                _))
            (else
              ;[1 1 1] More at halo? If looked at center, over, else under
              (if (and (> (Variables|Default|GethaloHits) (Variables|Default|GetcenterHits)) (> (Variables|Default|GetcenterHits) 0))
                (Math|Integer|IncrementInt _overshoots
                  (:%20%20
                    _))
                (else
                  (Math|Integer|IncrementInt _undershoots
                    (:%20%20
                      _))))))
          (Development|PrintString (Utilities|String|Append "Perfect: " (Utilities|String|ToString(Integer) _perfect) " Over Shoots: " (Utilities|String|ToString(Integer) _overshoots) " Under Shoots: " (Utilities|String|ToString(Integer) _undershoots)))
          (Variables|Default|SetCount (Variables|Default|GetMaxCount))
          (Variables|Default|SetcenterHits 0)
          (Variables|Default|SethaloHits 0)
          (Class|ListenerInt|ListenedActorIsDone(Message) (Variables|Default|GetparentActor) self))))))

(event Custom|EyesightTrackWasLost)

(event Custom|EyetrackWasFullyLost)

(event Custom|DisableActiveMode
  (Variables|Default|SetisActive false)
  (Rendering|SetVisibility (Variables|Default|Gethalo) false false))

(event Custom|EnableActiveMode
  (bind _datacollector (Variables|Default|GetdataCollector))
  (bind _datacollector_2 (Variables|Default|GetdataCollector))
  (bind _datacollector_3 (Variables|Default|GetdataCollector))
  (bind _datacollector_4 (Variables|Default|GetdataCollector))
  (bind _datacollector_5 (Variables|Default|GetdataCollector))
  (bind _badhits (Variables|/Game/OpeyeIIContent/Core/Gameplay/Actors/Saccades_A_StimulusDataCollector_Bp.Saccades_A_StimulusDataCollector_Bp_C|GetbadHits _datacollector_2))
  (bind _goodhits (Variables|/Game/OpeyeIIContent/Core/Gameplay/Actors/Saccades_A_StimulusDataCollector_Bp.Saccades_A_StimulusDataCollector_Bp_C|GetgoodHits _datacollector))
  (bind _undershoots (Variables|/Game/OpeyeIIContent/Core/Gameplay/Actors/Saccades_A_StimulusDataCollector_Bp.Saccades_A_StimulusDataCollector_Bp_C|GetunderShoots _datacollector_4))
  (bind _overshoots (Variables|/Game/OpeyeIIContent/Core/Gameplay/Actors/Saccades_A_StimulusDataCollector_Bp.Saccades_A_StimulusDataCollector_Bp_C|GetoverShoots _datacollector_5))
  (bind _perfect (Variables|/Game/OpeyeIIContent/Core/Gameplay/Actors/Saccades_A_StimulusDataCollector_Bp.Saccades_A_StimulusDataCollector_Bp_C|Getperfect _datacollector_3))
  (Variables|Default|SetisActive true)
  (Variables|Default|SetCount (Variables|Default|GetMaxCount))
  (Rendering|SetVisibility (Variables|Default|Gethalo) true false)
  (Utilities|FlowControl|Sequence
    (:then_0
      (bind _systemsave (CallFunction|GetSystemSave))
      (bind _output_get (Variables|Default|SetCount (Variables|/Game/OpeyeIIContent/Core/Data/System_Save.System_Save_C|GetA_Time_Variable _systemsave)))
      (Variables|Default|SetMaxCount _output_get)
      ;[1 0.4656 0] Timer for good hits or bad hits
      (Utilities|Time|SetTimerbyEvent (delegate Custom|Countdown) 1.0 true))
    (:then_1
      (Utilities|FlowControl|DoOnce true) ; enters at Reset
    )))

(event Custom|Countdown
  ;[1 0.4656 0] Timer for good hits or bad hits
  (if (> (Variables|Default|GetCount) 0)
    (Math|Integer|DecrementInt (Variables|Default|GetCount))))

(event EventBeginPlay
  (bind _hitmanager_cmp (Variables|Default|GetHitManager_Cmp))
  (bind _systemsave (CallFunction|GetSystemSave))
  (switch Utilities|FlowControl|Switch|SwitchonSizes_Enum (Variables|/Game/OpeyeIIContent/Core/Data/System_Save.System_Save_C|GetA_Size _systemsave)
    (:NewEnumerator0
      (Variables|Default|Setsize "1.000000,1.000000,1.000000"))
    (:NewEnumerator1
      (Variables|Default|Setsize "1.300000,1.300000,1.300000"))
    (:NewEnumerator2
      (Variables|Default|Setsize "1.600000,1.600000,1.600000")))
  (Utilities|FlowControl|Sequence
    (:then_0
      (if (not (Variables|Default|GetisActive))
        (Rendering|SetVisibility (Variables|Default|Gethalo) false false)))
    (:then_1
      (EventDispatchers|BindEventtoTrackLossWarning _hitmanager_cmp (delegate Custom|EyesightTrackWasLost))
      (EventDispatchers|BindEventtoExerciseComplete _hitmanager_cmp (delegate Custom|ExerciseWasCompleted))
      (EventDispatchers|BindEventtoStartedBeingTracked _hitmanager_cmp (delegate Custom|EyesightIsTrackingMeAgain))
      (EventDispatchers|BindEventtoTrackFullyLostWarning _hitmanager_cmp (delegate Custom|EyetrackWasFullyLost))
      (Transformation|SetActorScale3D (Variables|Default|Getsize)))))

(event Collision|EventActorBeginOverlap
  (params (OtherActor :type Actor%20Object%20Reference)))

(event EventTick
  (params (DeltaSeconds :type Float%20%28single-precision%29)))

(event EventSetParent
  (params (Actor :type Actor%20Object%20Reference))
  (Variables|Default|SetparentActor Actor))

(event EventHit
  (params (Hit%20Component%20Name :type String))
  (if (Variables|Default|GetisActive)
    ;[1 1 1] Add hits to each collision
    (switch string Hit%20Component%20Name
      (:Center
        (Math|Integer|IncrementInt (Variables|Default|GetcenterHits)
          (:%20%20
            _)))
      (:halo
        (Math|Integer|IncrementInt (Variables|Default|GethaloHits)
          (:%20%20
            _))))
    (Default|ManageHit (Variables|Default|GetHitManager_Cmp))))

(fn ConstructionScript)

(fn GetSystemSave
  (Utilities|IsValid (Variables|Default|GetSystem)
    (:Is%20Valid
      (return (Variables|Default|GetSystem)))
    (:Is%20Not%20Valid
      (bind _returnvalue (SaveGame|DoesSaveGameExist (CallFunction|GetSystemSaveName)))
      (if _returnvalue
        (bind _returnvalue_2 (SaveGame|LoadGamefromSlot (CallFunction|GetSystemSaveName)))
        (bind _assystem_save (Utilities|Casting|CastToSystem_Save _returnvalue_2)
          (:then
            (Variables|Default|SetSystem _assystem_save))
          (:CastFailed
            _))
        (else
          (bind _returnvalue_3 (SaveGame|CreateSaveGameObject "/Game/OpeyeIIContent/Core/Data/System_Save.System_Save_C"))
          (Variables|Default|SetSystem _returnvalue_3)))
      (return (Variables|Default|GetSystem)))))

(fn GetTarget
  (return 0))
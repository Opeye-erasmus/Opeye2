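; Spawner that fills a box area with a grid of Platform_Bp actors on BeginPlay.
; The construction script sizes the box, and the reset function destroys existing platforms, then interpolates row and column positions across its X/Y extent at the box center's height.
; Each spawn gets an Id, random yaw and random scale, and joins ChildrenPlatforms.
; Lookup functions return the start platform by Id 0, and the next and last by array order.
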(event EventBeginPlay
  (CallFunction|ResetAllPlatforms))

(event Collision|EventActorBeginOverlap
  (params (OtherActor :type Actor%20Object%20Reference)))

(event EventTick
  (params (DeltaSeconds :type Float%20%28single-precision%29)))

(fn ConstructionScript
  (Components|Box|SetBoxExtent (Variables|Default|GetExtend) (Variables|Default|GetAreaExtend) true))

(fn SpawnPlatform
  (params (id :type Integer) (location :type Vector))
  (bind _randomscale (Variables|Default|GetRandomScale))
  (bind _random_rotation (Variables|Default|Getrandom%20rotation))
  (bind _returnvalue (* _randomscale -1.0))
  (bind _returnvalue_2 (Game|SpawnActorfromClass "/Game/OpeyeIIContent/Core/Gameplay/Platform_Bp.Platform_Bp_C" (Math|Transform|MakeTransform location (Math|Rotator|MakeRotator 0.0 0.0 (Math|Random|RandomFloatinRange (* _random_rotation -1.0) _random_rotation)) (* (Variables|Default|GetBaseScale) (+ (Math|Random|RandomFloatinRange (Math|Float|Min(Float) _randomscale _returnvalue) (Math|Float|Max(Float) _randomscale _returnvalue)) 1.0))) "Undefined" 0 0))
  (Variables|/Game/OpeyeIIContent/Core/Gameplay/Platform_Bp.Platform_Bp_C|Setid _returnvalue_2 id)
  (Utilities|Array|AddUnique (Variables|Default|GetchildrenPlatforms) _returnvalue_2))

(fn DeleteAllChildrenPlatforms
  (bind _childrenplatforms (Variables|Default|GetchildrenPlatforms))
  (for _array_element _childrenplatforms
    (Actor|DestroyActor _array_element))
  (Utilities|Array|Clear _childrenplatforms))

(fn ResetAllPlatforms
  (bind _extend (Variables|Default|GetExtend))
  (bind _extend_2 (Variables|Default|GetExtend))
  (bind _numberofrows (Variables|Default|GetnumberOfRows))
  (bind _numberofcols (Variables|Default|GetnumberOfCols))
  (bind _returnvalue (Transformation|GetWorldLocation _extend))
  (bind _returnvalue_2 (- _numberofrows 1))
  (bind _returnvalue_3 (- _numberofcols 1))
  (bind _returnvalue_4 (Transformation|GetWorldLocation _extend_2))
  (bind _boxextent (Variables|/Script/Engine.BoxComponent|GetBoxExtent _extend))
  (bind _boxextent_2 (Variables|/Script/Engine.BoxComponent|GetBoxExtent _extend_2))
  (bind (_x _y _z) (Math|Vector|BreakVector _returnvalue_4))
  (bind (_x_2 _y_2) (Math|Vector|BreakVector _boxextent))
  (bind (_x_3 _y_3 _z_2) (Math|Vector|BreakVector _returnvalue))
  (bind (_x_4 _y_4) (Math|Vector|BreakVector _boxextent_2))
  (CallFunction|DeleteAllChildrenPlatforms)
  (LocalVariables|SetInitialLocation (Math|Vector|MakeVector (- _x _x_4) (- _y _y_4) _z))
  (LocalVariables|SetFinalLocation (Math|Vector|MakeVector (+ _x_3 _x_2) (+ _y_3 _y_2) _z_2))
  (if (and (> (Variables|Default|GetnumberOfRows) 0) (> (Variables|Default|GetnumberOfCols) 0))
    (for _index (range 0 _returnvalue_2)
      (for _index_2 (range 0 _returnvalue_3)
        (CallFunction|SpawnPlatform (Variables|Default|Getindex) (Math|Vector|MakeVector (+ (.X (Math|Vector|BreakVector (LocalVariables|GetInitialLocation))) (/ (* _index_2 (- (.X (Math|Vector|BreakVector (LocalVariables|GetFinalLocation))) (.X (Math|Vector|BreakVector (LocalVariables|GetInitialLocation))))) (Math|Conversions|ToFloat(Integer) _returnvalue_3))) (+ (.Y (Math|Vector|BreakVector (LocalVariables|GetInitialLocation))) (/ (* _index (- (.Y (Math|Vector|BreakVector (LocalVariables|GetFinalLocation))) (.Y (Math|Vector|BreakVector (LocalVariables|GetInitialLocation))))) (Math|Conversions|ToFloat(Integer) _returnvalue_2))) (.Z (Math|Vector|BreakVector (LocalVariables|GetFinalLocation)))))
        (Math|Integer|IncrementInt (Variables|Default|Getindex))))))

(fn GiveMeStartPlatform
  (for _array_element (Variables|Default|GetchildrenPlatforms)
    (if (== (Variables|/Game/OpeyeIIContent/Core/Gameplay/Platform_Bp.Platform_Bp_C|Getid _array_element) 0)
      (return _array_element)))
  (return 0))

(fn FindNextPlatform
  (params (CurrentPlatform :type Platform%20Bp%20Object%20Reference))
  (bind _childrenplatforms (Variables|Default|GetchildrenPlatforms))
  (bind (_array_element _array_index) (Utilities|Array|ForEachLoopwithBreak _childrenplatforms :!label _label)
    (:LoopBody
      (if (== _array_element CurrentPlatform)
        (bind _output_get (LocalVariables|SetNextId _array_index))
        (Development|PrintString (Utilities|String|ToString(Integer) _output_get))
        (goto _label Break)))
    (:Completed
      (if (Utilities|Array|IsValidIndex _childrenplatforms (LocalVariables|GetNextId))
        (return (Utilities|Array|Get(acopy) _childrenplatforms (+ (LocalVariables|GetNextId) 1)))
        (else
          (return 0))))))

(fn GiveMeLastPlatform
  (bind _childrenplatforms (Variables|Default|GetchildrenPlatforms))
  (if (> (Utilities|Array|Length _childrenplatforms) 0)
    (return (Utilities|Array|Get(acopy) _childrenplatforms (Utilities|Array|LastIndex _childrenplatforms)))
    (else
      (return 0))))
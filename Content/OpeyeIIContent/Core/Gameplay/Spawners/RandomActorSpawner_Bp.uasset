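; Spawner actor that places a set number of actors, each drawn randomly from a class list, automatically on BeginPlay or through SpawnNewObjects.
; The construction script sizes a box volume from Extent; spawns land randomly inside it or at its center, with optional random rotation and random uniform scale.
; The validity check and spawn roll the class separately, so they can differ.
; Spawned actors are tracked for destruction by DestroyMySpawnedActors.
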(event Custom|DestroyMySpawnedActors
  (bind _spawnedactors (Variables|Default|GetspawnedActors))
  (for _array_element _spawnedactors
    (Actor|DestroyActor _array_element))
  (Utilities|Array|Clear _spawnedactors))

(event Custom|SpawnNewObjects
  (bind _volume (Variables|Default|GetVolume))
  (bind _actorclasstospawn (Variables|Default|GetActorClassToSpawn))
  (bind _returnvalue (Utilities|Array|Length _actorclasstospawn))
  (bind _returnvalue_2 (Transformation|GetWorldLocation _volume))
  (bind _returnvalue_3 (- _returnvalue 1))
  (bind _returnvalue_4 (Math|Random|RandomIntegerinRange 0 _returnvalue_3))
  (bind _output (Utilities|Array|Get(acopy) _actorclasstospawn _returnvalue_4))
  (for _index (range 0 (- (Variables|Default|GetAmountOfActors) 1))
    (if (Utilities|IsValidClass _output)
      (bind _returnvalue_5 (Game|SpawnActorfromClass _output (Math|Transform|MakeTransform (Math|Vector|SelectVector (Math|Random|RandomPointinBoundingBox _returnvalue_2 (Variables|/Script/Engine.BoxComponent|GetBoxExtent _volume)) _returnvalue_2 (Variables|Default|GetrandomSpawnLocation)) (Math|Rotator|SelectRotator (Math|Random|RandomRotator true) "0, 0, 0" (Variables|Default|GetuseRandomRotation)) (* "1.000000,1.000000,1.000000" (Math|Random|RandomFloatinRange (Variables|Default|GetMinSizeScale) (Variables|Default|GetMaxSizeScale)))) "Undefined" 0 0))
      (Utilities|Array|AddUnique (Variables|Default|GetspawnedActors) _returnvalue_5))))

(event EventBeginPlay
  (if (Variables|Default|GetautoSpawn)
    (CallFunction|SpawnNewObjects)))

(event Collision|EventActorBeginOverlap
  (params (OtherActor :type Actor%20Object%20Reference)))

(event EventTick
  (params (DeltaSeconds :type Float%20%28single-precision%29)))

(fn ConstructionScript
  (Components|Box|SetBoxExtent (Variables|Default|GetVolume) (Variables|Default|GetExtent) true))
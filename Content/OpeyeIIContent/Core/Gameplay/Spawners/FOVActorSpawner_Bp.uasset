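; Spawner for a field-of-view exercise that alternates a central fixation stimulus with randomly placed targets.
; Completing the central stimulus spawns a save-scaled target in one of four quadrant boxes, drawn evenly from a shuffle-bag and nudged off-center, or at recorded positions when replaying.
; Target callbacks record success or timeout, accumulate seek time and re-arm the center via a DoOnce.
; An empty bag ends the game through FOV_Pwn; positions and results feed a target report.
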(event Custom|DestroyMySpawnedActors
  (params (Stimulus :type Static%20Stimulus%20Bp%20Object%20Reference) (Material :type Material%20Object%20Reference))
  (bind _centralstimulus (Variables|Default|GetCentralStimulus))
  (bind _volumestospawn (Variables|Default|GetvolumesToSpawn))
  (Variables|Default|SetstimulusSpawned false)
  (Variables|Default|SetmeanTimeToSeekStimulus (+ (Variables|/Game/OpeyeIIContent/Core/Gameplay/Actors/StaticStimulus_Bp.StaticStimulus_Bp_C|GettimeElapsed Stimulus) (Variables|Default|GetmeanTimeToSeekStimulus)))
  (Rendering|Material|SetMaterial (Variables|/Game/OpeyeIIContent/Core/Gameplay/Actors/StaticStimulus_Bp.StaticStimulus_Bp_C|GetSphere Stimulus) 0 Material)
  (Default|StopTimer Stimulus)
  (Rendering|SetActorHiddenInGame Stimulus true)
  (Variables|/Game/OpeyeIIContent/Core/Gameplay/Actors/StaticStimulus_Bp.StaticStimulus_Bp_C|Setviewed Stimulus true)
  (Variables|/Game/OpeyeIIContent/Core/Gameplay/Actors/StaticStimulus_Bp.StaticStimulus_Bp_C|Setviewed _centralstimulus false)
  (Default|ResetCache _centralstimulus)
  (Utilities|FlowControl|DoOnce false) ; enters at Reset
)

(event Custom|StaticStimReachedTimeout
  (params (Stimulus :type Static%20Stimulus%20Bp%20Object%20Reference))
  (Utilities|Array|SetArrayElem (Variables|Default|GetstimulusSuccess) (- (Variables|Default|GetstimulusSpawnedIndex) 1) false)
  (CallFunction|DestroyMySpawnedActors Stimulus "/Game/OpeyeIIContent/Art/Props/Wardrobe/clothes/Res/Red_Mat.Red_Mat"))

(event Custom|ShowStartStimulus
  (Utilities|IsValid (Variables|Default|GetCentralStimulus)
    (:Is%20Not%20Valid
      ;[1 1 1] Place new stimulus in the world
      (bind _returnvalue (Game|SpawnActorfromClass "/Game/OpeyeIIContent/Core/Gameplay/Actors/StaticStimulus_Bp.StaticStimulus_Bp_C" (Transformation|GetActorTransform) "Undefined" 0 0))
      (Variables|Default|SetCentralStimulus _returnvalue)
      (Variables|/Game/OpeyeIIContent/Core/Gameplay/Actors/StaticStimulus_Bp.StaticStimulus_Bp_C|Setflags _returnvalue -1)
      (Class|ChildInt|SetParent(Message) _returnvalue self)
      (Default|ChangeHaloVisibility _returnvalue true))))

(event Custom|SpawnNewObjects
  (bind _volumestospawn (Variables|Default|GetvolumesToSpawn))
  (Utilities|FlowControl|DoOnce false
    (:Completed
      (Variables|Default|SetstimulusSpawned true)
      (Math|Integer|IncrementInt (Variables|Default|GetstimulusSpawnedIndex)
        (:%20%20
          (if (Variables|Default|GetisReplaying)
            (bind _returnvalue (Game|SpawnActorfromClass (Variables|Default|GetActorClassToSpawn) (Math|Transform|MakeTransform (Utilities|Array|Get(acopy) (Variables|Default|GetstimulusPositions) (Variables|Default|Getindex)) (Math|Rotator|SelectRotator (Math|Random|RandomRotator true) "0, 0, 0" (Variables|Default|GetuseRandomRotation)) (Variables|Default|Getscale)) "Undefined" 0 0))
            (Math|Integer|IncrementInt (Variables|Default|Getindex)
              (:%20%20
                (Utilities|Array|AddUnique (Variables|Default|GetspawnedActors) _returnvalue)
                (Class|ChildInt|SetParent(Message) _returnvalue self)))
            (else
              ;[1 1 1] Select random volume
              (if (> (Utilities|Array|Length _volumestospawn) 0)
                (bind _output_get (Variables|Default|SetcurrentVolumeIndex (.OutIndex (Utilities|Array|Random _volumestospawn))))
                (switch int (Utilities|Array|Get(acopy) _volumestospawn _output_get)
                  (:0
                    (Variables|Default|SetCurrentVolumeRef (Variables|Default|GetVolume_TL)))
                  (:1
                    (Variables|Default|SetCurrentVolumeRef (Variables|Default|GetVolume_TR)))
                  (:2
                    (Variables|Default|SetCurrentVolumeRef (Variables|Default|GetVolume_BL)))
                  (:3
                    (Variables|Default|SetCurrentVolumeRef (Variables|Default|GetVolume_BR))))
                ;[1 1 1] Remove from the stack
                (Utilities|Array|RemoveIndex (Variables|Default|GetvolumesToSpawn) (Variables|Default|GetcurrentVolumeIndex))
                ;[1 1 1] Place new stimulus in the world
                (bind _returnvalue_2 (Game|SpawnActorfromClass (Variables|Default|GetActorClassToSpawn) (Math|Transform|MakeTransform (CallFunction|AddDistancefromOrigin (Math|Random|RandomPointinBoundingBox (Transformation|GetWorldLocation (Variables|Default|GetCurrentVolumeRef)) (Variables|/Script/Engine.BoxComponent|GetBoxExtent (Variables|Default|GetCurrentVolumeRef)))) (Math|Rotator|SelectRotator (Math|Random|RandomRotator true) "0, 0, 0" (Variables|Default|GetuseRandomRotation)) (Variables|Default|Getscale)) "Undefined" 0 0))
                (Utilities|Array|Add (Variables|Default|GetstimulusPositions) (Transformation|GetActorLocation _returnvalue_2))
                (Utilities|Array|AddUnique (Variables|Default|GetspawnedActors) _returnvalue_2)
                (Class|ChildInt|SetParent(Message) _returnvalue_2 self)
                (else
                  ;[1 1 1] Finished  spawning elements
                  (Development|PrintString (Utilities|String|Append "Mean Time to Seek Stimulus: " (Utilities|String|ToString(Float) (/ (Variables|Default|GetmeanTimeToSeekStimulus) (Math|Conversions|ToFloat(Integer) (* (Variables|Default|GetMaxActorsToSpawnPerVolume) 4))))))
                  (Development|PrintString (Utilities|String|Append "Time elapsed in exercise: " (Utilities|String|ToString(Float) (Variables|Default|GettimeElapsed))))
                  (bind _asfov_pwn (Utilities|Casting|CastToFOV_Pwn (Game|Player|GetPlayerPawn 0)))
                  (Default|GameIsOver _asfov_pwn))))))))))

(event EventBeginPlay
  (bind _systemsave (CallFunction|GetSystemSave))
  (switch Utilities|FlowControl|Switch|SwitchonSizes_Enum (Variables|/Game/OpeyeIIContent/Core/Data/System_Save.System_Save_C|GetA_Size _systemsave)
    (:NewEnumerator0
      (Variables|Default|Setscale "0.500000,0.500000,0.500000"))
    (:NewEnumerator1
      (Variables|Default|Setscale "0.700000,0.700000,0.700000"))
    (:NewEnumerator2
      (Variables|Default|Setscale "1.300000,1.300000,1.300000")))
  (if (Variables|Default|GetautoSpawn)
    (for _index (range 1 (Variables|Default|GetMaxActorsToSpawnPerVolume))
      ;[1 1 1] we add one item to show per volume. This is repeated "maxActorsToSpawnPerVolume" times
      (Utilities|Array|Add (Variables|Default|GetvolumesToSpawn) 0)
      (Utilities|Array|Add (Variables|Default|GetvolumesToSpawn) 1)
      (Utilities|Array|Add (Variables|Default|GetvolumesToSpawn) 2)
      (Utilities|Array|Add (Variables|Default|GetvolumesToSpawn) 3))
    (for _index_2 (range 1 (* (Variables|Default|GetMaxActorsToSpawnPerVolume) 4))
      (Utilities|Array|Add (Variables|Default|GetstimulusSuccess) false))
    (CallFunction|ShowStartStimulus)))

(event EventTick
  (params (DeltaSeconds :type Float%20%28single-precision%29))
  (if (Variables|Default|GetstimulusSpawned)
    (Variables|Default|SettimeElapsed (+ DeltaSeconds (Variables|Default|GettimeElapsed)))))

(event EventListenedActorIsFullyLost
  (params (listenedActor :type Actor%20Object%20Reference))
  (bind _asstatic_stimulus_bp (Utilities|Casting|CastToStaticStimulus_Bp listenedActor))
  ;[1 1 1] if it is not the central stimulus
  (if (not (< (Variables|/Game/OpeyeIIContent/Core/Gameplay/Actors/StaticStimulus_Bp.StaticStimulus_Bp_C|Getflags _asstatic_stimulus_bp) 0))
    (Variables|/Game/OpeyeIIContent/Core/Gameplay/Actors/StaticStimulus_Bp.StaticStimulus_Bp_C|Setviewed (Variables|Default|GetCentralStimulus) false)
    (CallFunction|DestroyMySpawnedActors _asstatic_stimulus_bp "/Game/OpeyeIIContent/Art/Props/Wardrobe/clothes/Res/Green_Mat.Green_Mat")))

(event EventListenedActorIsDone
  (params (listenedActor :type Actor%20Object%20Reference))
  (bind _asstatic_stimulus_bp (Utilities|Casting|CastToStaticStimulus_Bp listenedActor))
  (if (< (Variables|/Game/OpeyeIIContent/Core/Gameplay/Actors/StaticStimulus_Bp.StaticStimulus_Bp_C|Getflags _asstatic_stimulus_bp) 0)
    ;[1 1 1] If the actor was the central stimulus, destroy and spawn a new target to look at
    (CallFunction|SpawnNewObjects)
    (Development|PrintString "Central asks for new objects")
    (Variables|/Game/OpeyeIIContent/Core/Gameplay/Actors/StaticStimulus_Bp.StaticStimulus_Bp_C|Setviewed (Variables|Default|GetCentralStimulus) true)
    (else
      ;[1 1 1] If the actor was not the central one, delete and show the central target
      (Utilities|Array|SetArrayElem (Variables|Default|GetstimulusSuccess) (- (Variables|Default|GetstimulusSpawnedIndex) 1) true)
      (CallFunction|DestroyMySpawnedActors _asstatic_stimulus_bp "/Game/OpeyeIIContent/Art/Props/Wardrobe/clothes/Res/Green_Mat.Green_Mat"))))

(fn ConstructionScript
  (bind _extent (Variables|Default|GetExtent))
  (bind _extent_2 (Variables|Default|GetExtent))
  (bind _extent_3 (Variables|Default|GetExtent))
  (bind _extent_4 (Variables|Default|GetExtent))
  (bind (_x _y _z) (Math|Vector|BreakVector _extent_2))
  (bind (_x_2 _y_2 _z_2) (Math|Vector|BreakVector _extent_3))
  (bind (_x_3 _y_3 _z_3) (Math|Vector|BreakVector _extent_4))
  (bind (_x_4 _y_4 _z_4) (Math|Vector|BreakVector _extent))
  (Components|Box|SetBoxExtent (Variables|Default|GetVolume_TL) (Variables|Default|GetExtent) true)
  (Transformation|SetRelativeLocation (Variables|Default|GetVolume_TL) (Math|Vector|MakeVector 0.0 (* _y -1.0) _z) false false)
  (Transformation|SetRelativeLocation (Variables|Default|GetVolume_TR) (Math|Vector|MakeVector 0.0 _y_3 _z_3) false false)
  (Transformation|SetRelativeLocation (Variables|Default|GetVolume_BL) (Math|Vector|MakeVector 0.0 (* _y_2 -1.0) (* _z_2 -1.0)) false false)
  (Transformation|SetRelativeLocation (Variables|Default|GetVolume_BR) (Math|Vector|MakeVector 0.0 _y_4 (* _z_4 -1.0)) false false))

(fn AddDistancefromOrigin
  (params (A :type Vector))
  (bind (_x _y _z) (Math|Vector|BreakVector A))
  (bind (_x_2 _y_2 _z_2) (Math|Vector|BreakVector A))
  (if (and (< _y 1e+02) (> _y -1e+02))
    (if (> _y 0.0)
      (LocalVariables|SetaddY 1e+02)
      (else
        (LocalVariables|SetaddY -1e+02)))
    (if (and (< _z 4e+02) (> _z 2e+02))
      (if (> _z 3e+02)
        (LocalVariables|SetaddZ 1e+02)
        (else
          (LocalVariables|SetaddZ -1e+02)))))
  (return (Math|Vector|MakeVector _x_2 (+ _y_2 (LocalVariables|GetaddY)) (+ _z_2 (LocalVariables|GetaddZ)))))

(fn GetTargetReport
  (for (_array_element _array_index) (Variables|Default|GetstimulusPositions)
    (Utilities|Array|Add (LocalVariables|GettargetReport) (Utilities|Struct|MakeTargetResultInfo_Str _array_element (Utilities|Array|Get(acopy) (Variables|Default|GetstimulusSuccess) _array_index))))
  (return (LocalVariables|GettargetReport)))

(fn PrintStimulusSuccess
  (bind _stimulussuccess (Variables|Default|GetstimulusSuccess))
  (for _array_element _stimulussuccess
    (if _array_element
      (Development|PrintString "bien")
      (else
        (Development|PrintString "mal"))))
  (Development|PrintString (Utilities|String|Append "Number of items: " (Utilities|String|ToString(Integer) (Utilities|Array|Length _stimulussuccess)))))
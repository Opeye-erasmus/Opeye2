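; Spawner for the Saccade word exercise that lays out a word as a row of linked, dash-masked Letter_bp actors.
; Random words come from Words_DT, filtered by profile language and a saved, clamped length, with spacing scaled by the saved size.
; The active spawner starts first and times its word.
; CanEnd loads collector data, then tries ending a Saccade game and triggers the next spawner, or chains preset words for other pawns.
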(event Custom|CanEnd
  (params (letterIndex :type Integer))
  ;[1 1 1] Is the letter index the same number as the length of the word?
  (if (>= letterIndex (- (Utilities|String|Len (Variables|Default|GetWord)) 1))
    ;[1 1 1] If yes, try to end the game, if you can't, spawn a new word using the next word spawner
    (Variables|Default|SetisDone true)
    (Default|LoadData (Variables|Default|GetdataCollector))
    (bind _assaccade_pwn (Utilities|Casting|CastToSaccade_Pwn (Game|Player|GetPlayerPawn 0))
      (:then
        (Default|TryEndGame _assaccade_pwn)
        (bind _nextwordspawner (Variables|Default|GetNextWordSpawner)
          (:then
            (CallFunction|SpawnRandomWord _nextwordspawner))
          (:else)))
      (:CastFailed
        (bind _nextwordspawner_2 (Variables|Default|GetNextWordSpawner)
          (:then
            (Variables|WordSpawner_Bp_C|SetisActive _nextwordspawner_2 true)
            (CallFunction|SpawnSelectedWord _nextwordspawner (Variables|WordSpawner_Bp_C|GetWord _nextwordspawner_2)))
          (:else
            (Class|ListenerInt|ListenedActorIsDone(Message) (Game|Player|GetPlayerPawn 0))))))))

(event Custom|Init
  ;[1 1 1] If the spawner is active at the begin, it means it is the first, so it spawns the first word
  (if (Variables|Default|GetisActive)
    (Utilities|Casting|CastToSaccade_Pwn (Game|Player|GetPlayerPawn 0))
    (CallFunction|SpawnRandomWord)))

(event EventBeginPlay
  ;[1 1 1] If the spawner is active at the begin, it means it is the first, so it spawns the first word
  (bind _outactors (Actor|GetAllActorsOfClass "/Game/OpeyeIIContent/Core/Gameplay/Pawn/Saccade_Pwn.Saccade_Pwn_C"))
  (Variables|Default|SetSaccadePwn (Utilities|Array|Get(acopy) _outactors))
  (CallFunction|Init))

(event EventTick
  (params (DeltaSeconds :type Float%20%28single-precision%29))
  (if (Variables|Default|GetisActive)
    (if (not (Variables|Default|GetisDone))
      (Variables|Default|SettimeElapsed (+ DeltaSeconds (Variables|Default|GettimeElapsed))))))

(fn ConstructionScript)

(fn CreateLetter
  (bind _returnvalue (Transformation|GetActorLocation))
  (bind (_x _y _z) (Math|Vector|BreakVector _returnvalue))
  (bind _returnvalue_2 (Game|SpawnActorfromClass "/Game/OpeyeIIContent/Core/Gameplay/Actors/Letter_bp.Letter_bp_C" (Math|Transform|MakeTransform (Math|Vector|MakeVector (+ (Variables|Default|GetAddSpace) _x) _y _z)) "Undefined" 0 0 0))
  (Development|PrintString (Utilities|String|ToString(Vector) (Math|Vector|MakeVector (+ (Variables|Default|GetAddSpace) _x) _y _z)))
  ;[1 1 1] Set index for the new LetterBp
  (Variables|/Game/OpeyeIIContent/Core/Gameplay/Actors/Letter_bp.Letter_bp_C|SetletterIndex _returnvalue_2 (Variables|Default|GetLetterIndex))
  ;[1 1 1] If there was an earlier letter, set the old LetterBp next letter to do the word sequence logic. If not, it is the first one, so set it as active
  (bind _letterbp (Variables|Default|GetLetterBp)
    (:then
      (Variables|/Game/OpeyeIIContent/Core/Gameplay/Actors/Letter_bp.Letter_bp_C|SetNextLetter _letterbp _returnvalue_2))
    (:else
      (Default|SetActiveColor _returnvalue_2)))
  (bind _output_get (Variables|Default|SetLetterBp _returnvalue_2))
  (Variables|/Game/OpeyeIIContent/Core/Gameplay/Actors/Letter_bp.Letter_bp_C|SetSpawner _output_get self)
  (bind _returnvalue_3 (CallFunction|GetLetter))
  (Variables|/Game/OpeyeIIContent/Core/Gameplay/Actors/Letter_bp.Letter_bp_C|SetLetter (Variables|Default|GetLetterBp) _returnvalue_3)
  (Rendering|Components|TextRender|SetText (Variables|/Game/OpeyeIIContent/Core/Gameplay/Actors/Letter_bp.Letter_bp_C|GetTextRender (Variables|Default|GetLetterBp)) (Utilities|Text|MakeLiteralText "-"))
  (Math|Integer|IncrementInt (Variables|Default|GetLetterIndex)
    (:%20%20
      (bind _systemsave (CallFunction|GetSystemSave))
      (Variables|Default|SetAddSpace (+ (* (Variables|Default|GetDistanceBetweenLetters) (Utilities|Select :Index (Variables|/Game/OpeyeIIContent/Core/Data/System_Save.System_Save_C|GetA_Size _systemsave) :NewEnumerator0 1.0 :NewEnumerator1 1.3 :NewEnumerator2 1.5)) (Variables|Default|GetAddSpace))))))

(fn SetStartingLocation
  (bind _systemsave (CallFunction|GetSystemSave)))

(fn SelectNewWord
  (bind _systemsave (CallFunction|GetSystemSave))
  (bind _output_get (LocalVariables|SetwordMaxLength (Math|Integer|Clamp(Integer) (Variables|/Game/OpeyeIIContent/Core/Data/System_Save.System_Save_C|GetAn_Amount_Of_Objects _systemsave) 3 8)))
  (bind _user_save (CallFunction|LoadUserProfile))
  (bind _words (CallFunction|FindListOfWords _output_get (Variables|/Game/OpeyeIIContent/Core/Data/UserProfile_Save.UserProfile_Save_C|Getlanguage _user_save)))
  (Variables|Default|SetWord (Utilities|String|GetSubstring (Utilities|String|ToString(Text) (.OutItem (Utilities|Array|Random _words))) 0 (LocalVariables|GetwordMaxLength))))

(fn GetLetter
  (bind _output_get (Variables|Default|SetLetter (Utilities|String|GetSubstring (Variables|Default|GetWord) (Variables|Default|GetLetterIndex))))
  (return (Utilities|Text|ToText(String) _output_get)))

(fn SpawnRandomWord
  ;[1 1 1] Create all the letters with * as placeholders
  (CallFunction|SelectNewWord)
  (CallFunction|SetStartingLocation)
  (for _index (range 0 (- (Utilities|String|Len (Variables|Default|GetWord)) 1))
    (CallFunction|CreateLetter)))

(fn SpawnSelectedWord
  (params (word :type String))
  (Variables|Default|SetWord word)
  (if (Variables|Default|GetisActive)
    (CallFunction|SetStartingLocation)
    (for _index (range 0 (- (Utilities|String|Len (Variables|Default|GetWord)) 1))
      (CallFunction|CreateLetter))))

(fn FindListOfWords
  (params (nOfLetters :type Integer) (language :type Languages_Enum%20Enum :default "NewEnumerator3"))
  (bind _outrownames (DataTable|GetDataTableRowNames "/Game/OpeyeIIContent/Data/Words_DT.Words_DT"))
  (for _array_element _outrownames
    (bind _returnvalue (Utilities|GetDataTableRow "/Game/OpeyeIIContent/Data/Words_DT.Words_DT" _array_element)
      (:then
        (if (and (== (.Length (Utilities|Struct|BreakWordInfo_Str _returnvalue)) nOfLetters) (Utilities|Enum|Equal(Enum) (.Language (Utilities|Struct|BreakWordInfo_Str _returnvalue)) language))
          (Utilities|Array|AddUnique (LocalVariables|GettempList) (.Word (Utilities|Struct|BreakWordInfo_Str _returnvalue)))))))
  (return (LocalVariables|GettempList)))
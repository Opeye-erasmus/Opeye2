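; Manager for the saccade exercise, which runs one pair of static stimuli chosen by the saved short- or long-distance setting.
; On BeginPlay it indexes stimuli by Id, hides the other pair, tints dynamic materials from the saved colour config and activates the first.
; Done messages alternate the active stimulus until the pair's second reaches the hit target.
; The HUD then shows good or bad from GoodHits, and the pawn is notified after a delay.
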(event EventBeginPlay
  (bind _systemsave (CallFunction|GetSystemSave))
  (bind _systemsave_2 (CallFunction|GetSystemSave))
  (bind _stimuli_refs (Variables|Default|GetStimuli_Refs))
  (bind _stimuli_refs_2 (Variables|Default|GetStimuli_Refs))
  (bind _typeofsaccade (Variables|/Game/OpeyeIIContent/Core/Data/System_Save.System_Save_C|GettypeOfSaccade _systemsave_2))
  (bind _typeofsaccade_2 (Variables|/Game/OpeyeIIContent/Core/Data/System_Save.System_Save_C|GettypeOfSaccade _systemsave))
  (bind _returnvalue (Utilities|Select :Index _typeofsaccade_2 :NewEnumerator0 0 :NewEnumerator1 2))
  (bind _output (Utilities|Array|Get(acopy) _stimuli_refs _returnvalue))
  (bind _returnvalue_2 (UserInterface|CreateWidget "/Game/OpeyeIIContent/Core/Interface/Saccades/Saccades_Result_Wgt.Saccades_Result_Wgt_C"))
  (bind _output_get (Variables|Default|SetHUD _returnvalue_2))
  (UserInterface|Viewport|AddtoViewport _output_get 0)
  (Utilities|FlowControl|Sequence
    (:then_0
      ;[1 1 1] Save space
      (Utilities|Array|Add _stimuli_refs_2 0)
      (Utilities|Array|Add _stimuli_refs_2 0)
      (Utilities|Array|Add _stimuli_refs_2 0)
      (Utilities|Array|Add _stimuli_refs_2 0))
    (:then_1
      (bind _outactors (Actor|GetAllActorsOfClass "/Game/OpeyeIIContent/Core/Gameplay/Actors/Saccades_A_StaticStimulus_Bp.Saccades_A_StaticStimulus_Bp_C"))
      (for _array_element _outactors
        (Utilities|FlowControl|Sequence
          (:then_0
            ;[1 1 1] Logic
            (Utilities|Array|SetArrayElem (Variables|Default|GetStimuli_Refs) (Variables|/Game/OpeyeIIContent/Core/Gameplay/Actors/Saccades_A_StaticStimulus_Bp.Saccades_A_StaticStimulus_Bp_C|Getid _array_element) _array_element)
            (Class|ChildInt|SetParent(Message) _array_element self)
            (if (or (== (Variables|/Game/OpeyeIIContent/Core/Gameplay/Actors/Saccades_A_StaticStimulus_Bp.Saccades_A_StaticStimulus_Bp_C|Getid _array_element) (Utilities|Select :Index _typeofsaccade :NewEnumerator0 2 :NewEnumerator1 0)) (== (Variables|/Game/OpeyeIIContent/Core/Gameplay/Actors/Saccades_A_StaticStimulus_Bp.Saccades_A_StaticStimulus_Bp_C|Getid _array_element) (Utilities|Select :Index _typeofsaccade :NewEnumerator0 3 :NewEnumerator1 1)))
              (Rendering|SetActorHiddenInGame _array_element true)))
          (:then_1
            ;[1 1 1] Set Ring Colour
            (bind _returnvalue_3 (Rendering|Material|CreateDynamicMaterialInstance "/Game/OpeyeIIContent/Art/Base/BaseMaterial.BaseMaterial" "None" "None" :!class /Script/Engine.KismetMaterialLibrary))
            (Variables|Default|Setmat _returnvalue_3)
            (Rendering|Material|SetMaterial (Variables|/Game/OpeyeIIContent/Core/Gameplay/Actors/Saccades_A_StaticStimulus_Bp.Saccades_A_StaticStimulus_Bp_C|Gethalo _array_element) 0 _returnvalue_3)
            (Rendering|Material|SetScalarParameterValue (Variables|Default|Getmat) "EmissiveInt" 1.0 :!class /Script/Engine.MaterialInstanceDynamic)
            (Rendering|Material|SetVectorParameterValue (Variables|Default|Getmat) "BaseColor" (Utilities|Select :Index (Variables|/Game/OpeyeIIContent/Core/Data/System_Save.System_Save_C|GetA_ColorConfig (CallFunction|GetSystemSave)) :NewEnumerator0 "(R=0.278894,G=1.000000,B=0.119538,A=1.000000)" :NewEnumerator1 "(R=1.000000,G=1.000000,B=1.000000,A=1.000000)" :NewEnumerator2 "(R=0.008568,G=0.127438,B=0.024158,A=1.000000)" :NewEnumerator3 "(R=0.913099,G=0.846873,B=0.000000,A=1.000000)" :NewEnumerator4 "(R=0.913099,G=0.846873,B=0.000000,A=1.000000)" :NewEnumerator5 "(R=1.000000,G=0.000000,B=0.000000,A=1.000000)" :NewEnumerator6 "(R=1.000000,G=1.000000,B=0.000000,A=1.000000)") :!class /Script/Engine.MaterialInstanceDynamic)
            (Rendering|Material|SetTextureParameterValue (Variables|Default|Getmat) "Texture" "/Game/OpeyeIIContent/Art/Props/Mat/Opeye_Halo.Opeye_Halo"))
          (:then_2
            ;[1 1 1] Set Sphere Colour
            (bind _returnvalue_4 (Rendering|Material|CreateDynamicMaterialInstance "/Game/OpeyeIIContent/Art/Base/BaseMaterial.BaseMaterial" "None" "None" :!class /Script/Engine.KismetMaterialLibrary))
            (Variables|Default|Setmat _returnvalue_4)
            (Rendering|Material|SetMaterial (Variables|/Game/OpeyeIIContent/Core/Gameplay/Actors/Saccades_A_StaticStimulus_Bp.Saccades_A_StaticStimulus_Bp_C|GetCenter _array_element) 0 _returnvalue_4)
            (Rendering|Material|SetScalarParameterValue (Variables|Default|Getmat) "EmissiveInt" 1.0 :!class /Script/Engine.MaterialInstanceDynamic)
            (Rendering|Material|SetVectorParameterValue (Variables|Default|Getmat) "BaseColor" (Utilities|Select :Index (Variables|/Game/OpeyeIIContent/Core/Data/System_Save.System_Save_C|GetA_ColorConfig (CallFunction|GetSystemSave)) :NewEnumerator0 "(R=0.278894,G=1.000000,B=0.119538,A=1.000000)" :NewEnumerator1 "(R=1.000000,G=1.000000,B=1.000000,A=1.000000)" :NewEnumerator2 "(R=0.008568,G=0.127438,B=0.024158,A=1.000000)" :NewEnumerator3 "(R=0.913099,G=0.846873,B=0.000000,A=1.000000)" :NewEnumerator4 "(R=0.913099,G=0.846873,B=0.000000,A=1.000000)" :NewEnumerator5 "(R=1.000000,G=0.000000,B=0.000000,A=1.000000)" :NewEnumerator6 "(R=1.000000,G=1.000000,B=0.000000,A=1.000000)") :!class /Script/Engine.MaterialInstanceDynamic)))))
    (:then_2
      ;[1 1 1] Set the stimulus to start with
      (Utilities|IsValid _output
        (:Is%20Valid
          (Default|EnableActiveMode _output))))))

(event EventListenedActorIsDone
  (params (listenedActor :type Actor%20Object%20Reference))
  (bind _stimuli_refs (Variables|Default|GetStimuli_Refs))
  (bind _hud (Variables|Default|GetHUD))
  (bind _stimuli_refs_2 (Variables|Default|GetStimuli_Refs))
  (bind _stimuli_refs_3 (Variables|Default|GetStimuli_Refs))
  (bind _stimuli_refs_4 (Variables|Default|GetStimuli_Refs))
  (bind _output (Utilities|Array|Get(acopy) _stimuli_refs_2 3))
  (bind _output_2 (Utilities|Array|Get(acopy) _stimuli_refs_3 1))
  (bind _output_3 (Utilities|Array|Get(acopy) _stimuli_refs_4))
  (bind _output_4 (Utilities|Array|Get(acopy) _stimuli_refs 2))
  (bind _assaccades_a_static_stimulus_bp (Utilities|Casting|CastToSaccades_A_StaticStimulus_Bp listenedActor))
  (if (>= (Variables|/Game/OpeyeIIContent/Core/Gameplay/Actors/Saccades_A_StaticStimulus_Bp.Saccades_A_StaticStimulus_Bp_C|GetnumberOfHits _assaccades_a_static_stimulus_bp) (Variables|Default|GetNumberOfSacadesToFinish))
    (switch int (Variables|/Game/OpeyeIIContent/Core/Gameplay/Actors/Saccades_A_StaticStimulus_Bp.Saccades_A_StaticStimulus_Bp_C|Getid _assaccades_a_static_stimulus_bp)
      (:0
        ;[1 1 1] Switch who is the active one -Activated when the stimulus is has to be seen more times
        (switch int (Variables|/Game/OpeyeIIContent/Core/Gameplay/Actors/Saccades_A_StaticStimulus_Bp.Saccades_A_StaticStimulus_Bp_C|Getid _assaccades_a_static_stimulus_bp) :!label _label
          (:0
            (Utilities|IsValid _output_2
              (:Is%20Valid
                (Default|EnableActiveMode _output_2))))
          (:1
            (Utilities|IsValid _output_3
              (:Is%20Valid
                (Default|EnableActiveMode _output_3))))
          (:2
            (Utilities|IsValid _output
              (:Is%20Valid
                (Default|EnableActiveMode _output))))
          (:3
            (Utilities|IsValid _output_4
              (:Is%20Valid
                (Default|EnableActiveMode _output_4))))))
      (:1
        ;[1 1 1] End resuts
        (if (> (Variables|/Game/OpeyeIIContent/Core/Gameplay/Actors/Saccades_A_StimulusDataCollector_Bp.Saccades_A_StimulusDataCollector_Bp_C|GetgoodHits (Variables|/Game/OpeyeIIContent/Core/Gameplay/Actors/Saccades_A_StaticStimulus_Bp.Saccades_A_StaticStimulus_Bp_C|GetdataCollector _assaccades_a_static_stimulus_bp)) 8) :!label _label_2
          (Default|ShowWell _hud)
          (else
            (Default|ShowBad _hud)))
        ;;[1 1 1] To ask the player finish the scene
        (Utilities|FlowControl|Delay 4.0)
        (Class|ListenerInt|ListenedActorIsDone(Message) (Game|Player|GetPlayerPawn 0) self))
      (:2
        (goto _label))
      (:3
        (goto _label_2)))
    (else
      (goto _label))))

(fn ConstructionScript)

(fn GetSystemSave
  (Utilities|IsValid (Variables|Default|GetSystem)
    (:Is%20Valid
      (return (Variables|Default|GetSystem)))
    (:Is%20Not%20Valid
      (bind _returnvalue (SaveGame|DoesSaveGameExist (CallFunction|GetSystemSaveName)))
      (if _returnvalue
        (bind _returnvalue_2 (SaveGame|LoadGamefromSlot (CallFunction|GetSystemSaveName)))
        (bind _assystem_save (Utilities|Casting|CastToSystem_Save _returnvalue_2)
          (:then
            (Variables|Default|SetSystem _assystem_save))
          (:CastFailed
            _))
        (else
          (bind _returnvalue_3 (SaveGame|CreateSaveGameObject "/Game/OpeyeIIContent/Core/Data/System_Save.System_Save_C"))
          (Variables|Default|SetSystem _returnvalue_3)))
      (return (Variables|Default|GetSystem)))))
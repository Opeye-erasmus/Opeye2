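; Fish aquarium actor with configurable water colour that relays eyesight focus to the fish.
; On BeginPlay it creates a dynamic water material and tints it with the colour preset from the cached System_Save, which is loaded or created on demand.
; Its Hit event loops over every Fish_Bp, notifying its own Fish that it receives eyesight and all others that they are ignored.
; GetTarget is an empty stub.
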(event EventBeginPlay
  ;[1 1 1] Set Water Colour
  (bind _returnvalue (Rendering|Material|CreateDynamicMaterialInstance (Variables|Default|GetStaticMesh) 0 "/Game/StarterContent/Materials/M_Water_Ocean_Inst.M_Water_Ocean_Inst" "None" :!class /Script/Engine.PrimitiveComponent))
  (Variables|Default|SetMat _returnvalue)
  (bind _systemsave (CallFunction|GetSystemSave))
  (Rendering|Material|SetVectorParameterValue (Variables|Default|GetMat) "Water Base Color" (Utilities|Select :Index (Variables|/Game/OpeyeIIContent/Core/Data/System_Save.System_Save_C|GetA_Water_Colour _systemsave) :NewEnumerator0 "" :NewEnumerator1 "(R=1.000000,G=1.000000,B=1.000000,A=1.000000)" :NewEnumerator2 "(R=0.854902,G=0.062745,B=0.145098,A=1.000000)" :NewEnumerator3 "(R=1.000000,G=0.941177,B=0.360784,A=1.000000)" :NewEnumerator4 "(R=0.113725,G=0.196078,B=0.329412,A=1.000000)" :NewEnumerator5 "(R=0.980392,G=1.000000,B=1.000000,A=1.000000)") :!class /Script/Engine.MaterialInstanceDynamic))

(event Collision|EventActorBeginOverlap
  (params (OtherActor :type Actor%20Object%20Reference)))

(event EventTick
  (params (DeltaSeconds :type Float%20%28single-precision%29)))

(event EventHit
  (params (Hit%20Component%20Name :type String))
  (bind _outactors (Actor|GetAllActorsOfClass "/Game/OpeyeIIContent/Core/Gameplay/Actors/Fish_Bp.Fish_Bp_C"))
  (for _array_element _outactors
    (if (== _array_element (Variables|Default|Getfish))
      (Default|ReceiveEyeSight _array_element)
      (else
        (Default|BeingIgnored _array_element)))))

(fn ConstructionScript)

(fn GetSystemSave
  (Utilities|IsValid (Variables|Default|GetSystem)
    (:Is%20Valid
      (return (Variables|Default|GetSystem)))
    (:Is%20Not%20Valid
      (bind _returnvalue (SaveGame|DoesSaveGameExist (CallFunction|GetSystemSaveName)))
      (if _returnvalue
        (bind _returnvalue_2 (SaveGame|LoadGamefromSlot (CallFunction|GetSystemSaveName)))
        (bind _assystem_save (Utilities|Casting|CastToSystem_Save _returnvalue_2)
          (:then
            (Variables|Default|SetSystem _assystem_save))
          (:CastFailed
            _))
        (else
          (bind _returnvalue_3 (SaveGame|CreateSaveGameObject "/Game/OpeyeIIContent/Core/Data/System_Save.System_Save_C"))
          (Variables|Default|SetSystem _returnvalue_3)))
      (return (Variables|Default|GetSystem)))))

(fn GetTarget
  (return 0))